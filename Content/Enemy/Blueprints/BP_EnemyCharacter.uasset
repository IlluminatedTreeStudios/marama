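; Enemy character that chases and melee-attacks the third-person player once the player overlaps it, and stops moving when the overlap ends.
; An AI MoveTo loop closes on the player, then plays an attack montage gated by a CanAttack cooldown.
; Damage is sent through TakeDamageMessage as the montage starts, not on an anim notify.
; When the montage completes, the chase resumes if the player is still in range.
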(event Custom|chase%20the%20player
  (AI|AIMoveTo self "0, 0, 0" (Game|GetPlayerCharacter 0) 1e+02 false
    (:OnSuccess
      (if (Variables|Default|Getcan_attack)
        (Variables|Default|Setcan_attack false)
        (Animation|Montage|PlayMontage (Variables|Character|GetMesh) "/Game/Enemy/Blueprints/AM_Enemy_Attack.AM_Enemy_Attack"
          (:then
            ;[1 1 1] Take Damage
            (Class|BPDamageable|TakeDamage(Message) (Game|GetPlayerCharacter 0) (Variables|Default|GetDmgToPlayer))
            (Utilities|FlowControl|Delay (Variables|Default|Getattack_rate))
            (Variables|Default|Setcan_attack true))
          (:OnCompleted
            (if (Variables|Default|Getplayer_in_range)
              (CallFunction|ChasethePlayer))))
        (else
          (CallFunction|ChasethePlayer))))))

(event Collision|EventActorBeginOverlap
  (params (OtherActor :type Actor%20Object%20Reference))
  (Utilities|Casting|CastToThirdPersonCharacter OtherActor)
  (Variables|Default|Setplayer_in_range true)
  (CallFunction|ChasethePlayer))

(event Collision|EventActorEndOverlap
  (params (OtherActor :type Actor%20Object%20Reference))
  (Utilities|Casting|CastToThirdPersonCharacter OtherActor)
  (Variables|Default|Setplayer_in_range false)
  (Components|Movement|StopMovementImmediately (Variables|Character|GetCharacterMovement)))

(fn ConstructionScript)