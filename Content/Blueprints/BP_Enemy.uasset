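; BP_Enemy is an enemy actor that loses health when hit and revives itself after reaching zero.
; Each hit on its Box subtracts a fixed amount of Health, regardless of the other actor.
; Tick polls for exactly zero Health, turns the Cube glowy red, then after a Delay turns it blue and resets Health.
; A TakeDamageMessage call to the other actor is present but never runs.
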(event OnComponentHit(Box)
  (params (HitComponent :type Primitive%20Component%20Object%20Reference) (OtherActor :type Actor%20Object%20Reference) (OtherComp :type Primitive%20Component%20Object%20Reference) (NormalImpulse :type Vector :default "0, 0, 0") (Hit :type Hit%20Result%20Structure%20%28by%20ref%29))
  (Variables|Default|Sethealth (- (Variables|Default|Gethealth) 2.5)))

(event EventTick
  (params (DeltaSeconds :type Float%20%28single-precision%29))
  (bind _cube (Variables|Default|GetCube))
  (if (== (Variables|Default|Gethealth) 0.0)
    (Rendering|Material|SetMaterial _cube 0 "/Game/Blueprints/M_Glowy_Red.M_Glowy_Red")
    (Utilities|FlowControl|Delay 1.0)
    (Rendering|Material|SetMaterial _cube 0 "/Game/Blueprints/M_Glowy_Blue.M_Glowy_Blue")
    (Variables|Default|Sethealth 5.0)))

(fn ConstructionScript)