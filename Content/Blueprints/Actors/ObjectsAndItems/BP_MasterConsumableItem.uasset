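; Master Blueprint for consumable items that resolves its own item data from the player's inventory component.
; On BeginPlay it runs SetItemProperties before calling the parent BeginPlay.
; That function casts player character 0 to BP_Player, searches BPCInventory's AvailableItems for an entry matching ItemName, and stores the first match as ItemStructure.
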(event EventBeginPlay
  (CallFunction|SetItemProperties)
  (|CallParentFunction))

(event Collision|EventActorBeginOverlap
  (params (OtherActor :type Actor%20Object%20Reference)))

(event EventTick
  (params (DeltaSeconds :type Float%20%28single-precision%29)))

(fn ConstructionScript
  (|CallParentFunction))

(fn SetItemProperties
  (bind _asbp_player (Utilities|Casting|CastToBP_Player (Game|GetPlayerCharacter 0)))
  (bind _array_element (Utilities|Array|ForEachLoopwithBreak (Variables|/Game/Blueprints/Actors/InventorySystem/BPC_Inventory.BPC_Inventory_C|GetAvailableItems (Variables|/Game/Blueprints/Player/BP_Player.BP_Player_C|GetBPC_Inventory _asbp_player)) :!label _label)
    (:LoopBody
      (bind _output_get (LocalVariables|SetArrayElement _array_element))
      (if (Utilities|Enum|Equal(Enum) (.Name (Utilities|Struct|BreakS_Items _output_get)) (Variables|Default|GetItemName))
        (Variables|Default|SetItemStructure self (LocalVariables|GetArrayElement))
        (goto _label Break)))
    (:Completed
      (return))))