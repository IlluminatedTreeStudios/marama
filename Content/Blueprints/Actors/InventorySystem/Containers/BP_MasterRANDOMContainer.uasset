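; BP_MasterRANDOMContainer is a master container Blueprint that holds randomized items and toggles its inventory on interaction.
; The construction script rolls each ItemTypes entry against its AppearanceProbability, adding a random quantity bounded by MaxStackSize until the slot count is reached.
; BeginPlay copies the generated Items into the ContainerInventory slots by index.
; Contents are rolled at construction time, before play begins.
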(event EventOnInteractwith
  (params (Player :type BP%20Player%20Object%20Reference))
  (Default|ToggleInventory (Variables|Default|GetContainer_Inventory)))

(event EventBeginPlay
  (for (_array_element _array_index) (Variables|Default|GetItems)
    (Utilities|Array|SetArrayElem (Variables|/Game/Blueprints/Actors/InventorySystem/BPC_Inventory.BPC_Inventory_C|GetInventory (Variables|Default|GetContainer_Inventory)) _array_index _array_element)))

(fn ConstructionScript
  ;[1 1 1] Inserts Random Items by probability
  (bind _array_element (Utilities|Array|ForEachLoopwithBreak (Variables|Default|GetItemTypes) :!label _label)
    (:LoopBody
      (if (and (Math|Random|RandomBoolwithWeight (.AppearanceProbability (Utilities|Struct|BreakS_Items _array_element))) (!= (Math|Random|RandomInteger (.MaxStackSize (Utilities|Struct|BreakS_Items _array_element))) 0))
        (Utilities|Array|Add (Variables|Default|GetItems) (Utilities|Struct|MakeS_Slots _array_element (Math|Random|RandomInteger (.MaxStackSize (Utilities|Struct|BreakS_Items _array_element)))))
        (bind _result (Math|Integer|IncrementInt (LocalVariables|GetSlotIndex))
          (:%20%20
            (if (>= _result (Variables|/Game/Blueprints/Actors/InventorySystem/BPC_Inventory.BPC_Inventory_C|GetNumberOfSlots (Variables|Default|GetContainer_Inventory)))
              (goto _label Break))))))))