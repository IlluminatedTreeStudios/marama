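; Loot container variant that fills itself with random items when play begins.
; It rolls each of the ContainerInventory's available items against its appearance probability and a second random check, then adds passing items to Items until the slot limit is reached.
; Quantities are re-rolled separately from that check and the debug print, capped by stack size or five, before the parent BeginPlay runs.
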(event EventBeginPlay
  (bind _array_element (Utilities|Array|ForEachLoopwithBreak (Variables|/Game/Blueprints/Actors/InventorySystem/BPC_Inventory.BPC_Inventory_C|GetAvailableItems (Variables|Default|GetContainer_Inventory)) :!label _label)
    (:LoopBody
      (if (and (Math|Random|RandomBoolwithWeight (.AppearanceProbability (Utilities|Struct|BreakS_Items _array_element))) (!= (Math|Random|RandomInteger (Math|Integer|Min(Integer) (.MaxStackSize (Utilities|Struct|BreakS_Items _array_element)) 5)) 0))
        (Development|PrintString (Utilities|String|ToString(Integer) (Math|Random|RandomInteger (Math|Integer|Min(Integer) (.MaxStackSize (Utilities|Struct|BreakS_Items _array_element)) 5))) true true "(R=0.000000,G=0.660000,B=1.000000,A=1.000000)" 1e+01)
        (Utilities|Array|Add (Variables|Default|GetItems) (Utilities|Struct|MakeS_Slots _array_element (+ (Math|Random|RandomInteger (Math|Integer|Min(Integer) (.MaxStackSize (Utilities|Struct|BreakS_Items _array_element)) 5)) 1)))
        (bind _result (Math|Integer|IncrementInt (Variables|Default|GetSlot%20Index))
          (:%20%20
            (if (>= _result (Variables|/Game/Blueprints/Actors/InventorySystem/BPC_Inventory.BPC_Inventory_C|GetNumberOfSlots (Variables|Default|GetContainer_Inventory)))
              (goto _label Break))))))
    (:Completed
      (|CallParentFunction))))

(fn ConstructionScript
  (|CallParentFunction))