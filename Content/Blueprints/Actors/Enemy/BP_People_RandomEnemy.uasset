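; Enemy character child Blueprint that gives each humanoid enemy a randomized appearance.
; The construction script runs the parent's, then picks random Head and Body skeletal meshes from the EnemyLook lists.
; It overrides SetHitAreaLocation without calling the parent, attaching HitArea to the left-hand socket for the first combo attack and the right-hand socket for the second.
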(fn ConstructionScript
  (bind _enemylook (Variables|Appearance|GetEnemyLook))
  (bind (_head _body) (Utilities|Struct|BreakS_EnemyLook _enemylook))
  (|CallParentFunction)
  (Class|SkinnedMeshComponent|SetSkeletalMesh (Variables|Default|GetHead) (.OutItem (Utilities|Array|Random _head)) true)
  (Class|SkinnedMeshComponent|SetSkeletalMesh (Variables|Character|GetMesh) (.OutItem (Utilities|Array|Random _body)) true))

(fn SetHitAreaLocation
  (if (== (Variables|Default|GetAttackComboIndex) 0) ; 1st Anim
    (Transformation|AttachComponentToComponent (Variables|Default|GetHitArea) (Variables|Character|GetMesh) "LH_S" "KeepRelative" "KeepRelative" "KeepRelative" true)
    (elif (== (Variables|Default|GetAttackComboIndex) 1) ; 2nd Anim
      (Transformation|AttachComponentToComponent (Variables|Default|GetHitArea) (Variables|Character|GetMesh) "RH_S" "KeepRelative" "KeepRelative" "KeepRelative" true))))