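; Player homing projectile with an invisible mesh material that steers toward enemies.
; From BeginPlay it repeats LockOn every half second, pointing ProjectileMovement's homing at the chosen enemy's scene component.
; FindHomingTarget scans all BP_MasterEnemy actors with a "dead" tag check and distance comparison meant to pick the closest.
; It assigns each passing element before comparing and never sets CurrentEnemy, so the pick may not be the nearest.
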(event Custom|Lock%20On
  (bind _projectilemovement (Variables|Default|GetProjectileMovement))
  (CallFunction|FindHomingTarget)
  (Utilities|IsValid (Variables|Default|GetClosestEnemy)
    (:Is%20Valid
      (Variables|/Script/Engine.ProjectileMovementComponent|SetHomingTargetComponent _projectilemovement (Actor|GetComponentbyClass (Variables|Default|GetClosestEnemy) "/Script/Engine.SceneComponent"))
      (Variables|/Script/Engine.ProjectileMovementComponent|SetbIsHomingProjectile _projectilemovement true))))

(event EventBeginPlay
  (|CallParentFunction)
  (CallFunction|Lockon :!label _label)
  (Utilities|FlowControl|Delay 0.5)
  (goto _label))

(event Collision|EventActorBeginOverlap
  (params (OtherActor :type Actor%20Object%20Reference)))

(event EventTick
  (params (DeltaSeconds :type Float%20%28single-precision%29)))

(fn ConstructionScript
  (|CallParentFunction)
  (Rendering|Material|SetMaterial (Variables|Character|GetMesh) 0 "/Game/Materials/Misc/M_Invisible.M_Invisible"))

(fn FindHomingTarget
  (bind _outactors (Actor|GetAllActorsOfClass "/Game/Blueprints/Actors/Enemy/BP_MasterEnemy.BP_MasterEnemy_C"))
  (for _array_element _outactors
    (if (not (Actor|ActorHasTag "dead"))
      (Variables|Default|SetClosestEnemy _array_element)
      (bind _output_get (LocalVariables|SetcurrentDistaneToEnemy (Math|Vector|VectorLength (- (Transformation|GetActorLocation) (Transformation|GetActorLocation)))))
      (if (< _output_get (Variables|Default|GetClosestDistance))
        (Variables|Default|SetClosestDistance (LocalVariables|GetcurrentDistaneToEnemy))
        (Variables|Default|SetClosestEnemy (LocalVariables|GetcurrentEnemy))))))