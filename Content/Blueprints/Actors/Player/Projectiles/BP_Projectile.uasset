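; BP_Projectile is a player projectile that damages enemies derived from BP_MasterEnemy and destroys itself on collision or when its lifetime expires.
; The construction script applies the mesh material and passes one Color to the projectile and spawn particle systems.
; On hit it prints a debug string, spawns the impact emitter's template at the impact point in that colour, and applies damage if the cast succeeds.
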(event OnComponentHit(collision)
  (params (HitComponent :type Primitive%20Component%20Object%20Reference) (OtherActor :type Actor%20Object%20Reference) (OtherComp :type Primitive%20Component%20Object%20Reference) (NormalImpulse :type Vector :default "0, 0, 0") (Hit :type Hit%20Result%20Structure%20%28by%20ref%29))
  (bind (_bblockinghit _binitialoverlap _time _distance _location _impactpoint _normal _impactnormal _physmat _hitactor) (Collision|BreakHitResult Hit))
  ;[1 1 1] Collision
  (Variables|Default|SetActorHit _hitactor)
  (Utilities|FlowControl|Sequence
    (:then_0
      (Development|PrintString "collision" false false))
    (:then_1
      (CallFunction|SpawnHitEffect _impactpoint))
    (:then_2
      (CallFunction|DamageEnemy (Variables|Default|GetActorHit)))
    (:then_3
      (Actor|DestroyActor) ; Destroy Projectile when hitting something
    )))

(event EventBeginPlay
  ;[1 1 1] BeginOfPlay
  (Utilities|FlowControl|Sequence
    (:then_1
      (Utilities|FlowControl|Delay (Variables|Default|GetDuration)) ; after certain time projectile \ngets destroyed
      (Actor|DestroyActor))))

(fn ConstructionScript
  (Effects|Components|ParticleSystem|SetColorParameter (Variables|Default|GetPS_Projectile) "Colour" (Variables|Default|GetColor))
  (Rendering|Material|SetMaterial (Variables|Default|GetMesh) 0 (Variables|Default|GetMaterial)))

(fn SpawnHitEffect
  (params (Location :type Vector%20%28by%20ref%29))
  (bind _returnvalue (Effects|SpawnEmitteratLocation (Variables|/Script/Engine.ParticleSystemComponent|GetTemplate (Variables|Default|GetPS_Impact)) Location))
  (Effects|Components|ParticleSystem|SetColorParameter _returnvalue "Colour" (Variables|Default|GetColor)))

(fn DamageEnemy
  (params (HitActor :type Actor%20Object%20Reference%20%28by%20ref%29))
  (bind _asbp_master_enemy (Utilities|Casting|CastToBP_MasterEnemy HitActor))
  (Game|Damage|ApplyDamage _asbp_master_enemy (Variables|Default|GetDamage) 0 0))