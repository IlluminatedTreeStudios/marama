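; Quest manager actor that spawns quest actors, tracks the selected quest and updates the HUD, journal and minimap.
; AddNewQuest rejects duplicate classes and auto-selects a first quest.
; Switching subgoals replaces the goal marker actor; player movement refreshes horizontal distance and arrow rotation, with paired DoOnce nodes toggling arrow visibility around a distance threshold.
; Enemy kills advance matching goals across all current quests, completing subgoals at their target count.
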(event EventBeginPlay)

(event Collision|EventActorBeginOverlap
  (params (OtherActor :type Actor%20Object%20Reference)))

(event EventTick
  (params (DeltaSeconds :type Float%20%28single-precision%29)))

(event Custom|OnSwitchSubQuest
  (bind _currentquest (Variables|Default|GetCurrentQuest))
  (bind _hud (Variables|Default|GetHUD))
  ;[1 1 1] Delete current SubGoal and set new one
  (Utilities|IsValid (Variables|Default|GetCurrentGoalActor)
    (:Is%20Valid
      (Actor|DestroyActor (Variables|Default|GetCurrentGoalActor)))
    (:Is%20Not%20Valid
      _))
  (bind _output_get (Variables|Default|SetCurrentSubGoal (Utilities|Array|Get(acopy) (.SubGoals (Utilities|Struct|BreakS_QuestInfo (Variables|/Game/Blueprints/Actors/QuestSystem/QuestActors/BP_MasterQuest.BP_MasterQuest_C|GetQuestInfo _currentquest))) (Variables|/Game/Blueprints/Actors/QuestSystem/QuestActors/BP_MasterQuest.BP_MasterQuest_C|GetSelectedSubGoalIndex _currentquest))))
  (if (.hasLocation (Utilities|Struct|BreakS_GoalLocation (.GoalLocation (Utilities|Struct|BreakS_GoalInfo _output_get))))
    (bind _returnvalue (Game|SpawnActorfromClass "/Game/Blueprints/Actors/QuestSystem/BP_GoalActor.BP_GoalActor_C" (Math|Transform|MakeTransform (.Location (Utilities|Struct|BreakS_GoalLocation (.GoalLocation (Utilities|Struct|BreakS_GoalInfo _output_get)))) "0, 0, 0" "1,1,1") "AlwaysSpawn" 0 (.UseRadius (Utilities|Struct|BreakS_GoalInfo _output_get)) (.Radius (Utilities|Struct|BreakS_GoalInfo _output_get)) (.CircleColor (Utilities|Struct|BreakS_GoalInfo _output_get)) 0)) ; Create GoalActor at Goal Location
    (Variables|Default|SetCurrentGoalActor _returnvalue)
    ;[1 1 1] Set Distance Value and Display in HUD
    (bind _output_get_2 (Variables|Default|SetCurrentDistance (CallFunction|DistancetoGoal)))
    (Rendering|Components|TextRender|SetText (Variables|/Game/Blueprints/UI/HUD/WBP_Main.WBP_Main_C|GetDistanceToQuestGoal (Variables|Default|GetHUD)) (Utilities|Text|ToText(Integer) _output_get_2 false false))
    (CallFunction|UpdateDirectionArrow)
    (Widget|SetVisibility (Variables|/Game/Blueprints/UI/HUD/WBP_Main.WBP_Main_C|GetDistanceBorder _hud) "HitTestInvisible")
    (Widget|SetVisibility (Variables|/Game/Blueprints/UI/HUD/WBP_MiniMap.WBP_MiniMap_C|GetDirectionArrow (Variables|/Game/Blueprints/UI/HUD/WBP_Main.WBP_Main_C|GetWBP_MiniMap _hud)) (select (> (Variables|Default|GetCurrentDistance) (Variables|Default|GetShowDirectionArrowAmount)) "HitTestInvisible" "Hidden"))
    (else
      ;[1 1 1] if new goal has no location, hide arrow
      (Variables|Default|SetCurrentGoalActor 0)
      (Widget|SetVisibility (Variables|/Game/Blueprints/UI/HUD/WBP_Main.WBP_Main_C|GetDistanceBorder (Variables|Default|GetHUD)) "Hidden"))))

(event Custom|OnPlayerMove
  (bind _hud (Variables|Default|GetHUD))
  (Utilities|IsValid (Variables|Default|GetCurrentGoalActor)
    (:Is%20Valid
      ;[1 1 1] set new distance after move
      (bind _output_get (Variables|Default|SetCurrentDistance (CallFunction|DistancetoGoal)))
      (Rendering|Components|TextRender|SetText (Variables|/Game/Blueprints/UI/HUD/WBP_Main.WBP_Main_C|GetDistanceToQuestGoal _hud) (Utilities|Text|ToText(Integer) _output_get false false))
      ;[1 1 1] check if player walks away from goal (after he was close) and displays arrow again
      (Math|Integer|CompareInt (Variables|Default|GetCurrentDistance) (Variables|Default|GetShowDirectionArrowAmount)
        (:>
          _)
        (:==
          _)
        (:<
          (Utilities|FlowControl|DoOnce false :!label _label
            (:Completed
              (Widget|SetVisibility (Variables|/Game/Blueprints/UI/HUD/WBP_MiniMap.WBP_MiniMap_C|GetDirectionArrow (Variables|/Game/Blueprints/UI/HUD/WBP_Main.WBP_Main_C|GetWBP_MiniMap _hud)) "Hidden")
              (goto _label_2 Reset)))))
      (CallFunction|UpdateDirectionArrow)
      (Utilities|FlowControl|DoOnce false :!label _label_2
        (:Completed
          (Widget|SetVisibility (Variables|/Game/Blueprints/UI/HUD/WBP_MiniMap.WBP_MiniMap_C|GetDirectionArrow (Variables|/Game/Blueprints/UI/HUD/WBP_Main.WBP_Main_C|GetWBP_MiniMap _hud)) "HitTestInvisible")
          (goto _label Reset))))))

(event Custom|OnEnemyKilled
  (params (Class :type BP%20Enemy%20Class%20Reference))
  (Variables|Default|SetKilledEnemy Class)
  (for _array_element (Variables|Default|GetCurrentQuestActors)
    (for (_array_element_2 _array_index) (Variables|/Game/Blueprints/Actors/QuestSystem/QuestActors/BP_MasterQuest.BP_MasterQuest_C|GetCurrentGoals _array_element)
      ;[1 0 0] hier könnte man abgleichen, um welchen type das pbjekt sich handelt und für alle quest arten gegenchecken
      (if (and (Utilities|Enum|Equal(Enum) (.Type (Utilities|Struct|BreakS_GoalInfo _array_element_2)) "NewEnumerator1") (== (.GoalClass (Utilities|Struct|BreakS_GoalInfo _array_element_2)) (Variables|Default|GetKilledEnemy)))
        (if (>= (+ (Utilities|Array|Get(acopy) (Variables|/Game/Blueprints/Actors/QuestSystem/QuestActors/BP_MasterQuest.BP_MasterQuest_C|GetCurrentHuntedOrGatheredAmount _array_element) _array_index) 1) (.AmountToHuntOrGather (Utilities|Struct|BreakS_GoalInfo _array_element_2))) ; check if amount to kill is reached
          (Default|CompleteSubGoal _array_element (Utilities|Array|Get(acopy) (Variables|/Game/Blueprints/Actors/QuestSystem/QuestActors/BP_MasterQuest.BP_MasterQuest_C|GetCurrentGoalIndices _array_element) _array_index))
          (else
            (Utilities|Array|SetArrayElem (Variables|/Game/Blueprints/Actors/QuestSystem/QuestActors/BP_MasterQuest.BP_MasterQuest_C|GetCurrentHuntedOrGatheredAmount _array_element) _array_index (+ (Utilities|Array|Get(acopy) (Variables|/Game/Blueprints/Actors/QuestSystem/QuestActors/BP_MasterQuest.BP_MasterQuest_C|GetCurrentHuntedOrGatheredAmount _array_element) _array_index) 1)) ; increment amount
            (Default|Update (Utilities|Array|Get(acopy) (Variables|/Game/Blueprints/UI/HUD/WBP_Quest.WBP_Quest_C|GetSubGoalWidget (Variables|/Game/Blueprints/Actors/QuestSystem/QuestActors/BP_MasterQuest.BP_MasterQuest_C|GetQuestWidget _array_element)) _array_index)) ; update in widget
            ;[1 1 1] if quest is selected, update subgoal in hud
            (if (Default|SelectinJournal _array_element)
              (Default|GenerateSubGoals (Variables|/Game/Blueprints/UI/HUD/WBP_Main.WBP_Main_C|GetWBP_QuestJournal (Variables|Default|GetHUD))))))))))

(fn ConstructionScript)

(fn SelectNewQuest
  (params (Quest :type BP%20Master%20Quest%20Object%20Reference) (SubGoal :type WBP%20Sub%20Goal%20Object%20Reference))
  (Utilities|IsValid (Variables|Default|GetCurrentQuest)
    (:Is%20Valid
      ;[1 1 1] disable current Quest and SubGoal
      (Widget|SetIsEnabled (Variables|/Game/Blueprints/UI/HUD/WBP_Quest.WBP_Quest_C|GetQuestName (Variables|/Game/Blueprints/Actors/QuestSystem/QuestActors/BP_MasterQuest.BP_MasterQuest_C|GetQuestWidget (Variables|Default|GetCurrentQuest))) false)
      (Default|SelectSubGoal (Variables|/Game/Blueprints/Actors/QuestSystem/QuestActors/BP_MasterQuest.BP_MasterQuest_C|GetQuestWidget (Variables|Default|GetCurrentQuest))))
    (:Is%20Not%20Valid
      _))
  ;[1 1 1] Set new current Quest
  (bind _output_get (Variables|Default|SetCurrentQuest Quest))
  (Default|OnQuestSelected (Variables|/Game/Blueprints/Actors/QuestSystem/QuestActors/BP_MasterQuest.BP_MasterQuest_C|GetQuestWidget _output_get) SubGoal)
  (return))

(fn AddNewQuest
  (params (QuestClass :type BP%20Master%20Quest%20Class%20Reference) (DirectlyStart :type Boolean))
  (LocalVariables|SetLocalClass QuestClass)
  (LocalVariables|SetLocalStart DirectlyStart)
  (if (and (Utilities|IsValidClass QuestClass) (not (Utilities|Array|ContainsItem (Variables|Default|GetAllQuestClasses) QuestClass)))
    (Utilities|Array|Add (Variables|Default|GetAllQuestClasses) (LocalVariables|GetLocalClass))
    (bind _returnvalue (Game|SpawnActorfromClass (LocalVariables|GetLocalClass) (Math|Transform|MakeTransform "0, 0, 0" "0, 0, 0" "1,1,1") "AlwaysSpawn" 0 self 0))
    (bind _output_get (LocalVariables|SetLocalQuestActor _returnvalue))
    (Utilities|Array|Add (Variables|Default|GetCurrentQuestActors) _output_get)
    (Default|SetUpStartingGoals _output_get)
    (bind _widget (Default|AddQuesttoList (Variables|Default|GetHUD) _output_get))
    (bind _output_get_2 (Variables|/Game/Blueprints/Actors/QuestSystem/QuestActors/BP_MasterQuest.BP_MasterQuest_C|SetQuestWidget _output_get _widget))
    (Default|UpdateQuest _output_get_2)
    (Default|AddEntry (Variables|/Game/Blueprints/UI/HUD/WBP_Main.WBP_Main_C|GetWBP_QuestJournal (Variables|Default|GetHUD)) _output_get)
    (if (or (LocalVariables|GetLocalStart) (<= (Utilities|Array|Length (Variables|Default|GetCurrentQuestActors)) 1))
      (CallFunction|SelectNewQuest _output_get (Utilities|Array|Get(acopy) (Variables|/Game/Blueprints/UI/HUD/WBP_Quest.WBP_Quest_C|GetSubGoalWidget (Variables|/Game/Blueprints/Actors/QuestSystem/QuestActors/BP_MasterQuest.BP_MasterQuest_C|GetQuestWidget _output_get))))
      (return true)
      (else
        (return true)))
    (else
      (return false))))

(fn DIstancetoGoal
  (bind _player (Variables|Default|GetPlayer))
  (bind _currentgoalactor (Variables|Default|GetCurrentGoalActor))
  (bind _returnvalue (Transformation|GetActorLocation _player))
  (bind _returnvalue_2 (Transformation|GetActorLocation _currentgoalactor))
  (return (Math|Conversions|ToInteger(Byte) (Class|KismetMathLibrary|Round64 (/ (Math|Vector|VectorLength (- (Math|Vector|MakeVector (.x _returnvalue) (.y _returnvalue) 0.0) (Math|Vector|MakeVector (.x _returnvalue_2) (.y _returnvalue_2) 0.0))) 1e+02)))))

(fn UpdateDirectionArrow
  (Class|Widget|SetRenderTransformAngle (Variables|/Game/Blueprints/UI/HUD/WBP_MiniMap.WBP_MiniMap_C|GetDirectionArrow (Variables|/Game/Blueprints/UI/HUD/WBP_Main.WBP_Main_C|GetWBP_MiniMap (Variables|Default|GetHUD))) (.Yaw (Math|Rotator|BreakRotator (Math|Rotator|FindLookatRotation (Transformation|GetActorLocation (Variables|Default|GetPlayer)) (Transformation|GetActorLocation (Variables|Default|GetCurrentGoalActor))))))
  (return))