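; Quest log component for the player that tracks accepted and active quests and toggles the quest journal widget on the HUD.
; Adding a quest credits collect objectives through its pickup call.
; Completion grants XP and regional prestige, detaches the quest actor from its NPC, refreshes NPCs cached at BeginPlay, and removes collected items.
; Helpers search an actor's attached quests by index and spawn objective enemies, though the spawn call on adding is disconnected.
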(event EventBeginPlay
  (bind _asbp_player (Utilities|Casting|CastToBP_Player (Components|GetOwner)))
  (Variables|Default|SetPlayer _asbp_player)
  (CallFunction|GetAllNPC))

(event EventTick
  (params (DeltaSeconds :type Float%20%28single-precision%29)))

(fn AddQuesttoLog
  (params (Quest :type A%20BP%20Master%20Quest%20Object%20Reference))
  (bind _quests (Variables|Default|GetQuests))
  ;[1 1 1] only add quest, if not in quest array
  (if (not (Utilities|Array|ContainsItem _quests Quest))
    (Utilities|Array|AddUnique _quests Quest)
    (Utilities|FlowControl|Sequence
      (:then_0
        ;[1 1 1] if collect qust, first check if item is already in inventory
        (for _array_element (Variables|/Game/Blueprints/Actors/QuestSystem/Quests/A_BP_MasterQuest.A_BP_MasterQuest_C|GetObjectives Quest)
          (if (Utilities|Enum|Equal(Enum) (.Type (Utilities|Struct|BreakS_ObjectiveData _array_element)) "NewEnumerator2")
            (bind _asbp_master_item (Utilities|Casting|CastToBP_MasterItem (.Target (Utilities|Struct|BreakS_ObjectiveData _array_element))))
            (Default|CallPickedUp Quest _asbp_master_item)))))))

(fn SetQuestActive
  (params (Quest :type A%20BP%20Master%20Quest%20Object%20Reference))
  (Utilities|IsValid (Variables|Default|GetActiveQuest)
    (:Is%20Valid
      _)
    (:Is%20Not%20Valid
      _))
  (bind _output_get (Variables|Default|SetActiveQuest Quest))
  (return _output_get))

(fn ToggleQuestJournal
  (bind _returnvalue (Game|GetPlayerCharacter 0))
  (bind _quest_journal (Variables|Default|GetQuest%20Journal)
    (:then
      (Widget|RemovefromParent _quest_journal)
      (Variables|Default|SetQuest%20Journal 0)
      (bind _asbp_player (Utilities|Casting|CastToBP_Player _returnvalue))
      (Default|ToggleInputMode _asbp_player))
    (:else
      (bind _asbp_player_2 (Utilities|Casting|CastToBP_Player (Game|GetPlayerCharacter 0)))
      (Default|CollapseAllJournals _asbp_player_2)
      (bind _returnvalue_2 (UserInterface|CreateWidget "/Game/Blueprints/UI/QuestJournal/WBP_QuestJournal.WBP_QuestJournal_C" 0 self))
      (Variables|Default|SetQuest%20Journal _returnvalue_2)
      (bind _asbp_player_3 (Utilities|Casting|CastToBP_Player _returnvalue))
      (Default|ToggleInputMode _asbp_player_3)
      (bind _returnvalue_3 (Class|CanvasPanel|AddChildtoCanvas (Variables|/Game/Blueprints/UI/HUD/WBP_Main.WBP_Main_C|GetHUD_Canvas (Variables|/Game/Blueprints/Player/BP_Player.BP_Player_C|GetHUD _asbp_player_3)) (Variables|Default|GetQuest%20Journal)))
      (Utilities|FlowControl|Sequence
        (:then_0
          (Class|CanvasPanelSlot|SetAnchors _returnvalue_3 (Utilities|Struct|MakeAnchors "(X=0.000000,Y=0.000000)" "(X=1.000000,Y=1.000000)")))
        (:then_1
          (Class|CanvasPanelSlot|SetZOrder _returnvalue_3 10))
        (:then_2
          (Class|CanvasPanelSlot|SetAlignment _returnvalue_3))
        (:then_3
          (Class|CanvasPanelSlot|SetOffsets _returnvalue_3))
        (:then_4
          (return))))))

(fn CompleteQuest
  (params (Quest :type A%20BP%20Master%20Quest%20Object%20Reference))
  (bind _output_get (LocalVariables|SetCompletedQuest Quest))
  (Variables|/Game/Blueprints/Actors/QuestSystem/Quests/A_BP_MasterQuest.A_BP_MasterQuest_C|SetCurrentState _output_get "NewEnumerator1")
  (Utilities|FlowControl|Sequence
    (:then_0
      ;[1 1 1] gain xp and prestige
      (bind _asbp_player (Utilities|Casting|CastToBP_Player (Game|GetPlayerCharacter 0)))
      (Default|AddXpPoints _asbp_player (Variables|/Game/Blueprints/Actors/QuestSystem/Quests/A_BP_MasterQuest.A_BP_MasterQuest_C|GetRewardXP (LocalVariables|GetCompletedQuest)))
      (Default|SetPrestigebyArea _asbp_player (Variables|/Game/Blueprints/Actors/QuestSystem/Quests/A_BP_MasterQuest.A_BP_MasterQuest_C|GetRegion (LocalVariables|GetCompletedQuest)) (Variables|/Game/Blueprints/Actors/QuestSystem/Quests/A_BP_MasterQuest.A_BP_MasterQuest_C|GetRewardPP (LocalVariables|GetCompletedQuest))))
    (:then_1
      ;[1 1 1] remove quest actor and check if npc has another quest
      (if (== (LocalVariables|GetCompletedQuest) (Variables|Default|GetActiveQuest))
        (Variables|Default|SetActiveQuest 0))
      (bind _asbp_master_people_npc (Utilities|Casting|CastToBP_MasterPeopleNPC (Actor|GetAttachParentActor (LocalVariables|GetCompletedQuest))))
      (Default|Update _asbp_master_people_npc)
      (Transformation|DetachFromActor (LocalVariables|GetCompletedQuest) "KeepRelative" "KeepRelative" "KeepRelative"))
    (:then_2
      ;[1 1 1] update all npc in world
      (for _array_element (Variables|Default|GetAllNPCsInWorld)
        (Default|Update _array_element)))
    (:then_3
      (bind _asbp_player_2 (Utilities|Casting|CastToBP_Player (Game|GetPlayerCharacter 0)))
      (for _array_element_2 (Variables|/Game/Blueprints/Actors/QuestSystem/Quests/A_BP_MasterQuest.A_BP_MasterQuest_C|GetObjectives (LocalVariables|GetCompletedQuest))
        (if (Utilities|Enum|Equal(Enum) (.type _array_element_2) "NewEnumerator2")
          (bind _asbp_master_item (Utilities|Casting|CastToBP_MasterItemClass (Utilities|GetClass (.target _array_element_2))))
          (Default|RemovefromInventory (Variables|/Game/Blueprints/Player/BP_Player.BP_Player_C|GetBPC_Inventory _asbp_player_2) _asbp_master_item (.number _array_element_2)))))))

(fn GetAllNPC
  (bind _outactors (Actor|GetAllActorsOfClass "/Game/Blueprints/NPC/BP_MasterPeopleNPC.BP_MasterPeopleNPC_C"))
  (Variables|Default|SetAllNPCsInWorld _outactors)
  (return))

(fn GetFirstQuestOfActor
  (params (Actor :type Actor%20Object%20Reference))
  (bind _outactors (Actor|GetAttachedActors Actor true))
  (Utilities|IsValid (Utilities|Array|Get(acopy) _outactors) ; does actor has attached objects?
    (:Is%20Valid
      (bind _output_get (LocalVariables|SetActors _outactors))
      (for (_array_element _array_index) _output_get
        (bind _asa_bp_master_quest (Utilities|Casting|CastToA_BP_MasterQuest _array_element))
        (if (< (Variables|/Game/Blueprints/Actors/QuestSystem/Quests/A_BP_MasterQuest.A_BP_MasterQuest_C|GetQuestIndex _asa_bp_master_quest) (LocalVariables|GetSmallestQuestIndex))
          (LocalVariables|SetSmallestQuestIndex (LocalVariables|GetSmallestQuestIndex))
          (LocalVariables|SetIndexActorWithSmallestIndex _array_index)
          (LocalVariables|SetHasQuest? true)))
      (if (LocalVariables|GetHasQuest?)
        (bind _asa_bp_master_quest_2 (Utilities|Casting|CastToA_BP_MasterQuest (Utilities|Array|Get(acopy) (LocalVariables|GetActors) (LocalVariables|GetIndexActorWithSmallestIndex)))))
      (return _asa_bp_master_quest_2 (LocalVariables|GetHasQuest?)))
    (:Is%20Not%20Valid
      (bind _output_get_2 (LocalVariables|SetHasQuest? false))
      (return 0 _output_get_2))))

(fn SpawnQuestEnemies
  (params (Objective :type S%20Objective%20Data%20Structure))
  (bind (_description _type _iscomplete_ _target _number _spawninfo) (Utilities|Struct|BreakS_ObjectiveData Objective))
  (bind (_spawnlocation _spawnactor _spawnradius _enemyname) (Utilities|Struct|BreakS_SpawnInfo _spawninfo))
  (for _index (range 1 _number)
    (bind _output_get (LocalVariables|SetNew (.RandomLocation (AI|Navigation|GetRandomReachablePointinRadius _spawnlocation _spawnradius 0 0))))
    (bind _returnvalue (Game|SpawnActorfromClass (Utilities|GetClass _spawnactor) (Math|Transform|MakeTransform _output_get "0, 0, 0" "1,1,1") "AdjustIfPossibleButAlwaysSpawn" 0 0))
    (bind _asbp_master_enemy (Utilities|Casting|CastToBP_MasterEnemy _returnvalue))
    (Variables|/Game/Blueprints/Enemy/BP_MasterEnemy.BP_MasterEnemy_C|SetNameOfEnemy _asbp_master_enemy _enemyname))
  (return))