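; Base pickup object the player collects by interacting with it, showing a name and "Press [E] to pick up" prompt.
; An InteractionRadius overlap shows or hides the prompt widget and sends enter and leave messages to the overlapped component's owner, the object itself.
; On interaction it adds its class to the player's ObtainedObjects, reports the find to the player's QuestManager and destroys itself.
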(event OnComponentBeginOverlap(InteractionRadius)
  (params (OverlappedComponent :type Primitive%20Component%20Object%20Reference) (OtherActor :type Actor%20Object%20Reference) (OtherComp :type Primitive%20Component%20Object%20Reference) (OtherBodyIndex :type Integer) (bFromSweep :type Boolean) (SweepResult :type Hit%20Result%20Structure%20%28by%20ref%29))
  ;[1 1 1] make widget visible by coming close to the object
  (Rendering|SetVisibility (Variables|Default|GetWidget) true false)
  (Class|BPIInteractNPC|OnEnterInteractionRadius(Message) (Components|GetOwner OverlappedComponent)))

(event OnComponentEndOverlap(InteractionRadius)
  (params (OverlappedComponent :type Primitive%20Component%20Object%20Reference) (OtherActor :type Actor%20Object%20Reference) (OtherComp :type Primitive%20Component%20Object%20Reference) (OtherBodyIndex :type Integer))
  ;[1 1 1] make widget visible by coming close to the object
  (Rendering|SetVisibility (Variables|Default|GetWidget) false false)
  (Class|BPIInteractNPC|OnLeaveInteractionRadius(Message) (Components|GetOwner OverlappedComponent)))

(event EventBeginPlay
  (bind _aswbp_interaction (Utilities|Casting|CastToWBP_Interaction (UserInterface|GetUserWidgetObject (Variables|Default|GetWidget))))
  (Rendering|Components|TextRender|SetText (Variables|/Game/Blueprints/UI/NPC/WBP_Interaction.WBP_Interaction_C|GetName _aswbp_interaction) (Variables|Default|GetName))
  (Rendering|Components|TextRender|SetText (Variables|/Game/Blueprints/UI/NPC/WBP_Interaction.WBP_Interaction_C|GetInteractionText _aswbp_interaction) "Press [E] to pick up"))

(event EventOnInteractwith
  (params (Player :type BP%20Player%20Object%20Reference))
  (bind _self self)
  (bind _returnvalue (Utilities|GetClass _self))
  (Utilities|Array|Add (Variables|/Game/Blueprints/Player/BP_Player.BP_Player_C|GetObtainedObjects Player) _returnvalue)
  (Default|OnObjectFound (Variables|/Game/Blueprints/Player/BP_Player.BP_Player_C|GetQuestManager Player) _returnvalue)
  (Actor|DestroyActor))

(fn ConstructionScript)