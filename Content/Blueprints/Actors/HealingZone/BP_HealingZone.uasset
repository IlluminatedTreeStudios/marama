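; BP_HealingZone is a scaled zone actor that marks the player as in a safezone or healing safezone.
; BeginPlay caches BP_Player, makes it the owner, and shows and scales the zone and its collision.
; Begin overlap adds Safezone.Healzone for active healing zones, otherwise plain Safezone, without checking which actor overlapped.
; End overlap removes only the Safezone tag; both overlaps toggle the player's darkness indicator.
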(event OnComponentBeginOverlap(CollisionZone)
  (params (OverlappedComponent :type Primitive%20Component%20Object%20Reference) (OtherActor :type Actor%20Object%20Reference) (OtherComp :type Primitive%20Component%20Object%20Reference) (OtherBodyIndex :type Integer) (bFromSweep :type Boolean) (SweepResult :type Hit%20Result%20Structure%20%28by%20ref%29))
  (bind _player (Variables|Default|GetPlayer))
  ;[1 1 1] Check: Player inside zone
  (Variables|Default|SetPlayerInside true)
  (if (Variables|Default|GetZoneActive)
    (if (Variables|Default|GetIsHealingZone)
      (Default|SetGameplayTag _player "(TagName=\"Safezone.Healzone\")" true)
      (else
        (Default|SetGameplayTag _player "(TagName=\"Safezone\")" true :!label _label)))
    (else
      (goto _label)))
  (Default|ToggleDarknessIndicator _player))

(event OnComponentEndOverlap(CollisionZone)
  (params (OverlappedComponent :type Primitive%20Component%20Object%20Reference) (OtherActor :type Actor%20Object%20Reference) (OtherComp :type Primitive%20Component%20Object%20Reference) (OtherBodyIndex :type Integer))
  (bind _player (Variables|Default|GetPlayer))
  (Variables|Default|SetPlayerInside false)
  ;[1 1 1] Check: Player inside zone
  (Utilities|IsValid _player
    (:Is%20Valid
      (Default|SetGameplayTag _player "(TagName=\"Safezone\")" false)
      (Default|ToggleDarknessIndicator _player))))

(event EventBeginPlay
  (bind _zone (Variables|Default|GetZone))
  (bind _scale (Variables|Default|GetScale))
  (bind _returnvalue (Math|Vector|MakeVector _scale _scale _scale))
  (bind _asbp_player (Utilities|Casting|CastToBP_Player (Game|GetPlayerCharacter 0)))
  (Variables|Default|SetPlayer _asbp_player)
  (Actor|SetOwner _asbp_player)
  (Rendering|SetVisibility _zone true false)
  (Transformation|SetRelativeScale3D _zone _returnvalue)
  (Transformation|SetRelativeScale3D (Variables|Default|GetCollisionZone) _returnvalue))

(fn ConstructionScript)