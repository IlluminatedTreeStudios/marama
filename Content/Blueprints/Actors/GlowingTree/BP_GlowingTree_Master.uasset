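; Base actor for a glowing tree the player revives by holding interact, granting a heal-zone gameplay tag removed on leaving.
; Collision overlap gates the interaction and shows a hold-to-interact widget.
; While held, a polled timer drives widget progress and a squared brightness ramp until a retriggerable delay activates or cancels the glow.
; Glow state switches the mark sprite and sick/happy label, with numpad debug toggles.
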(event OnComponentBeginOverlap(CollisionZone)
  (params (OverlappedComponent :type Primitive%20Component%20Object%20Reference) (OtherActor :type Actor%20Object%20Reference) (OtherComp :type Primitive%20Component%20Object%20Reference) (OtherBodyIndex :type Integer) (bFromSweep :type Boolean) (SweepResult :type Hit%20Result%20Structure%20%28by%20ref%29))
  ;[1 1 1] Check if player in interact radius
  (Variables|Default|SetPlayerInside true)
  (Development|PrintString "Entered TREE area" false)
  (CallFunction|ToggleWidget)
  ;[1 1 1] Main logic
  (Utilities|FlowControl|Gate true) ; enters at Open
)

(event OnComponentEndOverlap(CollisionZone)
  (params (OverlappedComponent :type Primitive%20Component%20Object%20Reference) (OtherActor :type Actor%20Object%20Reference) (OtherComp :type Primitive%20Component%20Object%20Reference) (OtherBodyIndex :type Integer))
  (bind _player (Variables|Default|GetPlayer))
  ;[1 1 1] Check if player in interact radius
  (Variables|Default|SetPlayerInside false)
  (Default|SetGameplayTag _player "(TagName=\"Safezone\")" false)
  (Default|SetGameplayTag _player "(TagName=\"Safezone.Healzone\")" false)
  (Development|PrintString "Left TREE area")
  (CallFunction|ToggleWidget)
  ;[1 1 1] Main logic
  (Utilities|FlowControl|Gate true) ; enters at Close
)

(event Custom|Timer
  ;[1 1 1] Timer logic for pressed key
  (bind _returnvalue (Utilities|Time|SetTimerbyEvent (delegate Custom|Timer) (Variables|Default|GetReviveTime))))

(event Custom|Stop%20Timer
  ;[1 1 1] Timer logic for pressed key
  (Utilities|Time|PauseTimerbyHandle (stale Custom|Timer _returnvalue)))

(event Custom|Update%20Timer
  (bind _keyheld (Variables|Default|GetKeyHeld))
  ;[1 1 1] Timer logic for pressed key
  (if (Math|Boolean|ANDBoolean (not (Variables|Default|GetZoneActive)) _keyheld (Variables|Default|GetPlayerInside))
    ;;[1 1 1] Gradualy increase glow
    (CallFunction|SetWidgetProgress (Class|KismetSystemLibrary|GetTimerElapsedTimeHandle (stale Custom|Timer _returnvalue)))
    (CallFunction|SetBrightness (Math|Float|Power (/ (Class|KismetSystemLibrary|GetTimerElapsedTimeHandle (stale Custom|Timer _returnvalue)) (Variables|Default|GetReviveTime)) 2.0))
    (Utilities|FlowControl|Delay 0.1)
    (CallFunction|UpdateTimer)
    (elif _keyheld
      (CallFunction|StopTimer)
      (CallFunction|SetWidgetProgress (Variables|Default|GetReviveTime))
      (else
        (CallFunction|StopTimer)
        (CallFunction|SetWidgetProgress 0.0)))))

(event EventBeginPlay
  (bind _treemark (Variables|Default|GetTreeMark))
  ;[1 1 1] Initialization
  (|CallParentFunction)
  (if (Variables|Default|GetZoneActive)
    (Rendering|Components|Sprite|SetSprite _treemark (Variables|Default|GetActiveSprite))
    (else
      (Rendering|Components|Sprite|SetSprite _treemark (Variables|Default|GetInactiveSprite))))
  (bind _aswbp_hold_interaction (Utilities|Casting|CastToWBP_HoldInteraction (UserInterface|GetUserWidgetObject (Variables|Default|GetHoldInteractionWidget))))
  (Rendering|Components|TextRender|SetText (Variables|/Game/Blueprints/UI/NPC/WBP_HoldInteraction.WBP_HoldInteraction_C|GetName _aswbp_hold_interaction) (Variables|Default|GetName))
  (Variables|/Game/Blueprints/UI/NPC/WBP_HoldInteraction.WBP_HoldInteraction_C|SetMaxTimeHeld _aswbp_hold_interaction (Variables|Default|GetReviveTime))
  (CallFunction|ToggleWidget))

(event EventOnInteractwith
  (params (Player :type BP%20Player%20Object%20Reference))
  ;[1 1 1] On Interaction
  (if (Collision|IsOverlappingActor (Variables|Default|GetInteractionZone) Player :!class /Script/Engine.PrimitiveComponent)
    (Variables|Default|SetKeyHeld true)
    (if (Variables|Default|GetZoneActive)
      (Development|PrintString "Tree already happy" false false)
      (CallFunction|Alreadyon)
      (else
        (Default|SetGameplayTag (Variables|Default|GetPlayer) "(TagName=\"Interaction.Tree\")" true)
        ;[1 1 1] Main logic
        (Utilities|FlowControl|Gate true
          (:Exit
            (Utilities|FlowControl|Sequence
              (:then_0
                (Utilities|FlowControl|RetriggerableDelay (Variables|Default|GetReviveTime))
                (if (Variables|Default|GetKeyHeld)
                  (CallFunction|EnableGlow)
                  (Utilities|FlowControl|Delay 0.5)
                  (CallFunction|ToggleWidget)
                  (else
                    (Animation|StopAnimMontage (Variables|Default|GetPlayer) "/Game/Animations/Player/MT_TreeInteract_V1.MT_TreeInteract_V1")
                    (CallFunction|DisableGlow))))
              (:then_1
                (CallFunction|Timer)
                (CallFunction|UpdateTimer)))))))))

(event EventOnInteractRelease
  ;[1 1 1] On Interaction
  (Default|SetGameplayTag (Variables|Default|GetPlayer) "(TagName=\"Interaction.Tree\")" false)
  (Variables|Default|SetKeyHeld false))

(event Input|KeyboardEvents|NumPadOne
  (params (Key :type Key%20Structure))
  (:Pressed
    (CallFunction|DisableGlow)
    (CallFunction|ToggleWidget)))

(event Input|KeyboardEvents|NumPadTwo
  (params (Key :type Key%20Structure))
  (:Pressed
    (CallFunction|EnableGlow)
    (CallFunction|ToggleWidget)))

(event Custom|EnableGlow
  (Variables|Default|SetZoneActive true)
  (Rendering|Components|Sprite|SetSprite (Variables|Default|GetTreeMark) (Variables|Default|GetActiveSprite))
  (Default|SetGameplayTag (Variables|Default|GetPlayer) "(TagName=\"Safezone.Healzone\")" (Variables|Default|GetZoneActive)))

(event Custom|DisableGlow
  (Variables|Default|SetZoneActive false)
  (Rendering|Components|Sprite|SetSprite (Variables|Default|GetTreeMark) (Variables|Default|GetInactiveSprite))
  (CallFunction|ToggleWidget)
  (Default|SetGameplayTag (Variables|Default|GetPlayer) "(TagName=\"Safezone.Healzone\")" (Variables|Default|GetZoneActive)))

(event Custom|SetBrightness
  (params (0%20to%201 :type Float%20%28single-precision%29))
  (Variables|Default|SetCurrentBrightness (* 0%20to%201 (Variables|Default|GetMaxBrightness))))

(fn ConstructionScript)

(fn SetWidgetProgress
  (params (Progress :type Float%20%28single-precision%29))
  (bind _aswbp_hold_interaction (Utilities|Casting|CastToWBP_HoldInteraction (UserInterface|GetWidget (Variables|Default|GetHoldInteractionWidget))))
  (bind _output_get (Variables|/Game/Blueprints/UI/NPC/WBP_HoldInteraction.WBP_HoldInteraction_C|SetTimeHeld _aswbp_hold_interaction Progress))
  (Default|SetProgress _aswbp_hold_interaction _output_get))

(fn ToggleWidget
  (bind _holdinteractionwidget (Variables|Default|GetHoldInteractionWidget))
  (bind _aswbp_hold_interaction (Utilities|Casting|CastToWBP_HoldInteraction (UserInterface|GetWidget _holdinteractionwidget)))
  (if (Variables|Default|GetZoneActive)
    (Rendering|Components|TextRender|SetText (Variables|/Game/Blueprints/UI/NPC/WBP_HoldInteraction.WBP_HoldInteraction_C|GetName _aswbp_hold_interaction) "Happy Tree")
    (Widget|SetVisibility (Variables|/Game/Blueprints/UI/NPC/WBP_HoldInteraction.WBP_HoldInteraction_C|GetCircleProgressBar _aswbp_hold_interaction) "Hidden")
    (Widget|SetVisibility (Variables|/Game/Blueprints/UI/NPC/WBP_HoldInteraction.WBP_HoldInteraction_C|GetInteractionText _aswbp_hold_interaction) "Hidden")
    (else
      (Rendering|Components|TextRender|SetText (Variables|/Game/Blueprints/UI/NPC/WBP_HoldInteraction.WBP_HoldInteraction_C|GetName _aswbp_hold_interaction) "Sick Tree")
      (Widget|SetVisibility (Variables|/Game/Blueprints/UI/NPC/WBP_HoldInteraction.WBP_HoldInteraction_C|GetCircleProgressBar _aswbp_hold_interaction) "Visible")
      (Widget|SetVisibility (Variables|/Game/Blueprints/UI/NPC/WBP_HoldInteraction.WBP_HoldInteraction_C|GetInteractionText _aswbp_hold_interaction) "Visible")))
  (if (Variables|Default|GetPlayerInside)
    (Rendering|SetVisibility _holdinteractionwidget true false)
    (else
      (Rendering|SetVisibility _holdinteractionwidget false false))))

(fn Alreadyon)