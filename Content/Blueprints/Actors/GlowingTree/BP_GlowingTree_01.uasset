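; BP_GlowingTree_01 is a glowing tree actor that extends a parent's glow behavior with its own material and four point lights.
; Construction creates a dynamic M_Glowy_Tree instance, whose base and light colors are randomized on BeginPlay and Alreadyon.
; Enable and disable glow events switch both material intensity and point lights, while SetBrightness updates only the material from CurrentBrightness.
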(event EventBeginPlay
  (bind _returnvalue (Math|Random|RandomFloatinRange 0.0 1.0))
  (bind _returnvalue_2 (Math|Random|RandomFloatinRange 0.0 1.0))
  (bind _returnvalue_3 (Math|Random|RandomFloatinRange 0.0 1.0))
  (bind _dynamicmaterial (Variables|Default|GetDynamicMaterial))
  (bind _linearcolor (Utilities|Struct|MakeLinearColor _returnvalue _returnvalue_2 _returnvalue_3 0.0))
  (|CallParentFunction)
  ;[1 1 1] Random color
  (Rendering|Material|SetVectorParameterValue _dynamicmaterial "BaseColor" _linearcolor :!class /Script/Engine.MaterialInstanceDynamic)
  (Rendering|Material|SetVectorParameterValue _dynamicmaterial "LightColor" _linearcolor :!class /Script/Engine.MaterialInstanceDynamic))

(event EventAlreadyon
  (bind _returnvalue (Math|Random|RandomFloatinRange 0.0 1.0))
  (bind _returnvalue_2 (Math|Random|RandomFloatinRange 0.0 1.0))
  (bind _returnvalue_3 (Math|Random|RandomFloatinRange 0.0 1.0))
  (bind _dynamicmaterial (Variables|Default|GetDynamicMaterial))
  (bind _linearcolor (Utilities|Struct|MakeLinearColor _returnvalue _returnvalue_2 _returnvalue_3 0.0))
  ;[1 1 1] Random color
  (Rendering|Material|SetVectorParameterValue _dynamicmaterial "BaseColor" _linearcolor :!class /Script/Engine.MaterialInstanceDynamic)
  (Rendering|Material|SetVectorParameterValue _dynamicmaterial "LightColor" _linearcolor :!class /Script/Engine.MaterialInstanceDynamic))

(event EventDisableGlow
  (|CallParentFunction)
  (Rendering|Material|SetScalarParameterValue (Variables|Default|GetDynamicMaterial) "Intensity" 0.0 :!class /Script/Engine.MaterialInstanceDynamic)
  (Rendering|Components|Light|SetIntensity (Variables|Default|GetPointLight) 0.0))

(event EventEnableGlow
  (|CallParentFunction)
  (Rendering|Material|SetScalarParameterValue (Variables|Default|GetDynamicMaterial) "Intensity" (Variables|Default|GetMaxBrightness) :!class /Script/Engine.MaterialInstanceDynamic)
  (Rendering|Components|Light|SetIntensity (Variables|Default|GetPointLight) 5e+03))

(event EventSetBrightness
  (params (0%20to%201 :type Float%20%28single-precision%29))
  (|CallParentFunction 0%20to%201)
  (Rendering|Material|SetScalarParameterValue (Variables|Default|GetDynamicMaterial) "Intensity" (Variables|Default|GetCurrentBrightness) :!class /Script/Engine.MaterialInstanceDynamic))

(fn ConstructionScript
  (|CallParentFunction)
  (bind _returnvalue (Rendering|Material|CreateDynamicMaterialInstance (Variables|Default|GetStaticMesh) 1 "/Game/Materials/DavidsKiste/M_Glowy_Tree.M_Glowy_Tree" "None" :!class /Script/Engine.PrimitiveComponent))
  (Variables|Default|SetDynamicMaterial _returnvalue))