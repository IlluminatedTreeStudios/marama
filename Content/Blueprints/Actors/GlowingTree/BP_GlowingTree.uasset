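; Glowing tree actor that the player revives by holding interact, turning a sick tree into a glowing healing zone.
; A collision sphere gates input and the hold widget, while a retriggerable delay enables or disables the glow depending on whether the key remains held.
; A timer-driven polling loop feeds widget progress and squared emission brightness on a dynamic material.
; Color randomizes at start and when interacting with a revived tree.
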(event OnComponentBeginOverlap(ColissionSphere)
  (params (OverlappedComponent :type Primitive%20Component%20Object%20Reference) (OtherActor :type Actor%20Object%20Reference) (OtherComp :type Primitive%20Component%20Object%20Reference) (OtherBodyIndex :type Integer) (bFromSweep :type Boolean) (SweepResult :type Hit%20Result%20Structure%20%28by%20ref%29))
  ;[1 1 1] Check if player in interact radius
  (Variables|Default|SetPlayerInside true)
  (Development|PrintString "Entered TREE area")
  (Utilities|Casting|CastToBP_Player OtherActor)
  (Input|EnableInput (Game|GetPlayerController 0))
  (CallFunction|ToggleWidget)
  ;[1 1 1] Main logic
  (Utilities|FlowControl|Gate true) ; enters at Open
)

(event OnComponentEndOverlap(ColissionSphere)
  (params (OverlappedComponent :type Primitive%20Component%20Object%20Reference) (OtherActor :type Actor%20Object%20Reference) (OtherComp :type Primitive%20Component%20Object%20Reference) (OtherBodyIndex :type Integer))
  ;[1 1 1] Check if player in interact radius
  (Variables|Default|SetPlayerInside false)
  (Development|PrintString "Left TREE area")
  (Utilities|Casting|CastToBP_Player OtherActor)
  (Input|DisableInput (Game|GetPlayerController 0))
  (CallFunction|ToggleWidget)
  ;[1 1 1] Main logic
  (Utilities|FlowControl|Gate true) ; enters at Close
)

(event Custom|Timer
  ;[1 1 1] Timer logic for pressed key
  (bind _returnvalue (Utilities|Time|SetTimerbyEvent (delegate Custom|Timer) (Variables|Default|GetReviveTime))))

(event Custom|Stop%20Timer
  ;[1 1 1] Timer logic for pressed key
  (Utilities|Time|PauseTimerbyHandle (stale Custom|Timer _returnvalue)))

(event Custom|Update%20Timer
  (bind _keyheld (Variables|Default|GetKeyHeld))
  ;[1 1 1] Timer logic for pressed key
  (if (Math|Boolean|ANDBoolean (not (Variables|Default|GetZoneActive)) _keyheld (Variables|Default|GetPlayerInside))
    ;;[1 1 1] Gradualy increase glow
    (CallFunction|SetWidgetProgress (Class|KismetSystemLibrary|GetTimerElapsedTimeHandle (stale Custom|Timer _returnvalue)))
    (CallFunction|SetBrightness (Math|Float|Power (/ (Class|KismetSystemLibrary|GetTimerElapsedTimeHandle (stale Custom|Timer _returnvalue)) (Variables|Default|GetReviveTime)) 2.0))
    (Utilities|FlowControl|Delay 0.1)
    (CallFunction|UpdateTimer)
    (elif _keyheld
      (CallFunction|StopTimer)
      (CallFunction|SetWidgetProgress (Variables|Default|GetReviveTime))
      (else
        (CallFunction|StopTimer)
        (CallFunction|SetWidgetProgress 0.0)))))

(event EventBeginPlay
  ;[1 1 1] Initialization
  (Utilities|FlowControl|Sequence
    (:then_0
      (Variables|Default|SetHealingAmount 2.0)
      (bind _aswbp_hold_interaction (Utilities|Casting|CastToWBP_HoldInteraction (UserInterface|GetUserWidgetObject (Variables|Default|GetHoldInteractionWidget))))
      (Rendering|Components|TextRender|SetText (Variables|/Game/Blueprints/UI/NPC/WBP_HoldInteraction.WBP_HoldInteraction_C|GetName _aswbp_hold_interaction) (Variables|Default|GetName))
      (Variables|/Game/Blueprints/UI/NPC/WBP_HoldInteraction.WBP_HoldInteraction_C|SetMaxTimeHeld _aswbp_hold_interaction (Variables|Default|GetReviveTime))
      (CallFunction|ToggleWidget))
    (:then_1
      ;[1 1 1] Random color
      (Rendering|Material|SetVectorParameterValue (Variables|Default|GetDynamic%20Material) "Color" (Utilities|Struct|MakeLinearColor (Math|Random|RandomFloatinRange 0.0 1.0) (Math|Random|RandomFloatinRange 0.0 1.0) (Math|Random|RandomFloatinRange 0.0 1.0) 1.0) :!class /Script/Engine.MaterialInstanceDynamic))))

(event EventOnInteractwith
  (params (Player :type BP%20Player%20Object%20Reference))
  ;[1 1 1] On Interaction
  (Variables|Default|SetKeyHeld true)
  (if (Variables|Default|GetZoneActive)
    (Development|PrintString "Tree already happy")
    ;[1 1 1] Random color
    (Rendering|Material|SetVectorParameterValue (Variables|Default|GetDynamic%20Material) "Color" (Utilities|Struct|MakeLinearColor (Math|Random|RandomFloatinRange 0.0 1.0) (Math|Random|RandomFloatinRange 0.0 1.0) (Math|Random|RandomFloatinRange 0.0 1.0) 1.0) :!class /Script/Engine.MaterialInstanceDynamic)
    (else
      ;[1 1 1] Main logic
      (Utilities|FlowControl|Gate true
        (:Exit
          (Utilities|FlowControl|Sequence
            (:then_0
              (Utilities|FlowControl|RetriggerableDelay (Variables|Default|GetReviveTime))
              (if (Variables|Default|GetKeyHeld)
                (CallFunction|EnableGlow)
                (Utilities|FlowControl|Delay 1.0)
                (CallFunction|ToggleWidget)
                (else
                  (CallFunction|DisableGlow))))
            (:then_1
              (CallFunction|Timer)
              (CallFunction|UpdateTimer))))))))

(event EventOnInteractRelease
  ;[1 1 1] On Interaction
  (Variables|Default|SetKeyHeld false))

(event Input|KeyboardEvents|NumPadOne
  (params (Key :type Key%20Structure))
  (:Pressed
    (CallFunction|DisableGlow)
    (CallFunction|ToggleWidget)))

(event Input|KeyboardEvents|NumPadTwo
  (params (Key :type Key%20Structure))
  (:Pressed
    (CallFunction|EnableGlow)
    (CallFunction|ToggleWidget)))

(fn ConstructionScript
  (bind _returnvalue (Rendering|Material|CreateDynamicMaterialInstance (Variables|Default|GetMesh) 1 "/Game/Materials/DavidsKiste/M_Emissive_David.M_Emissive_David" "None" :!class /Script/Engine.PrimitiveComponent))
  (Variables|Default|SetDynamic%20Material _returnvalue)
  (Variables|Default|SetIsHealingZone true))

(fn DisableGlow
  (Variables|Default|SetZoneActive false)
  (Rendering|Material|SetScalarParameterValue (Variables|Default|GetDynamic%20Material) "Emission" 0.0 :!class /Script/Engine.MaterialInstanceDynamic)
  (Rendering|Components|Sprite|SetSprite (Variables|Default|GetTreeMark) 0)
  (CallFunction|ToggleWidget)
  ;[1 1 1] todo: set Tag
  (Variables|/Game/Blueprints/Player/BP_Player.BP_Player_C|SetIsInHealingZone (Variables|Default|GetPlayer) false))

(fn EnableGlow
  (Variables|Default|SetZoneActive true)
  (Rendering|Material|SetScalarParameterValue (Variables|Default|GetDynamic%20Material) "Emission" (Variables|Default|GetMaxBrightness) :!class /Script/Engine.MaterialInstanceDynamic)
  (Rendering|Components|Sprite|SetSprite (Variables|Default|GetTreeMark) 0)
  ;[1 1 1] todo: set Tag
  (Variables|/Game/Blueprints/Player/BP_Player.BP_Player_C|SetIsInHealingZone (Variables|Default|GetPlayer) true))

(fn SetWidgetProgress
  (params (Progress :type Float%20%28single-precision%29))
  (bind _aswbp_hold_interaction (Utilities|Casting|CastToWBP_HoldInteraction (UserInterface|GetWidget (Variables|Default|GetHoldInteractionWidget))))
  (bind _output_get (Variables|/Game/Blueprints/UI/NPC/WBP_HoldInteraction.WBP_HoldInteraction_C|SetTimeHeld _aswbp_hold_interaction Progress))
  (Default|SetProgress _aswbp_hold_interaction _output_get))

(fn ToggleWidget
  (bind _holdinteractionwidget (Variables|Default|GetHoldInteractionWidget))
  (bind _aswbp_hold_interaction (Utilities|Casting|CastToWBP_HoldInteraction (UserInterface|GetWidget _holdinteractionwidget)))
  (if (Variables|Default|GetZoneActive)
    (Rendering|Components|TextRender|SetText (Variables|/Game/Blueprints/UI/NPC/WBP_HoldInteraction.WBP_HoldInteraction_C|GetName _aswbp_hold_interaction) "Happy Tree")
    (Widget|SetVisibility (Variables|/Game/Blueprints/UI/NPC/WBP_HoldInteraction.WBP_HoldInteraction_C|GetWBP_HoldInteract_CircleProgressBar _aswbp_hold_interaction) "Hidden")
    (Widget|SetVisibility (Variables|/Game/Blueprints/UI/NPC/WBP_HoldInteraction.WBP_HoldInteraction_C|GetInteractionText _aswbp_hold_interaction) "Hidden")
    (else
      (Rendering|Components|TextRender|SetText (Variables|/Game/Blueprints/UI/NPC/WBP_HoldInteraction.WBP_HoldInteraction_C|GetName _aswbp_hold_interaction) "Sick Tree")
      (Widget|SetVisibility (Variables|/Game/Blueprints/UI/NPC/WBP_HoldInteraction.WBP_HoldInteraction_C|GetWBP_HoldInteract_CircleProgressBar _aswbp_hold_interaction) "Visible")
      (Widget|SetVisibility (Variables|/Game/Blueprints/UI/NPC/WBP_HoldInteraction.WBP_HoldInteraction_C|GetInteractionText _aswbp_hold_interaction) "Visible")))
  (if (Variables|Default|GetPlayerInside)
    (Rendering|SetVisibility _holdinteractionwidget true false)
    (else
      (Rendering|SetVisibility _holdinteractionwidget false false))))

(fn SetBrightness
  (params (0_to_1 :type Float%20%28single-precision%29))
  (Rendering|Material|SetScalarParameterValue (Variables|Default|GetDynamic%20Material) "Emission" (* 0_to_1 (Variables|Default|GetMaxBrightness)) :!class /Script/Engine.MaterialInstanceDynamic))