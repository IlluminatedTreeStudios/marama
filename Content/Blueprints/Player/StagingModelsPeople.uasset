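; Staging model of a person, assembled from a body mesh and a head in the construction script.
; The Body asset is set on Mesh, and Head follows its pose as a master-pose child.
; Glowy puts BodyMaterial on both parts, creating a dynamic instance that is never applied; otherwise the head gets its own material.
; The event graph and ChangeAnimation are empty stubs.
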(event EventBeginPlay)

(event Collision|EventActorBeginOverlap
  (params (OtherActor :type Actor%20Object%20Reference)))

(event EventTick
  (params (DeltaSeconds :type Float%20%28single-precision%29)))

(fn ConstructionScript
  (Class|SkinnedMeshComponent|SetSkeletalMesh (Variables|Character|GetMesh) (Variables|Creating|GetBody) true)
  (Class|SkinnedMeshComponent|SetMasterPoseComponent (Variables|Default|GetHead) (Variables|Character|GetMesh) false)
  (if (Variables|Creating|GetGlowy?)
    (bind _returnvalue (Rendering|Material|CreateDynamicMaterialInstance (Variables|Creating|GetBodyMaterial) "None" "None" :!class /Script/Engine.KismetMaterialLibrary))
    (Rendering|Material|GetVectorParameterValue _returnvalue "LightColor" :!class /Script/Engine.MaterialInstanceDynamic)
    (Rendering|Material|SetMaterial (Variables|Character|GetMesh) 0 (Variables|Creating|GetBodyMaterial))
    (else
      (Rendering|Material|SetMaterial (Variables|Character|GetMesh) 0 (Variables|Creating|GetBodyMaterial))
      (Rendering|Material|SetMaterial (Variables|Default|GetHead) 0 (Variables|Default|GetHeadhMaterial)))))

(fn ChangeAnimation)