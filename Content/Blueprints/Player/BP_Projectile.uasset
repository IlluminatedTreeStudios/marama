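; BP_Projectile is a player projectile actor that damages enemies on impact and destroys itself on any hit or after a three-second lifetime.
; Collision hits print a debug string, spawn a particle at the impact point and apply damage only to BP_MasterEnemy actors.
; An unconnected SetGlowyMaterial helper would create a dynamic material and match the point light's color to it, but never runs.
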(event OnComponentHit(collision)
  (params (HitComponent :type Primitive%20Component%20Object%20Reference) (OtherActor :type Actor%20Object%20Reference) (OtherComp :type Primitive%20Component%20Object%20Reference) (NormalImpulse :type Vector :default "0, 0, 0") (Hit :type Hit%20Result%20Structure%20%28by%20ref%29))
  (bind (_bblockinghit _binitialoverlap _time _distance _location _impactpoint _normal _impactnormal _physmat _hitactor) (Collision|BreakHitResult Hit))
  ;[1 1 1] Collision
  (Variables|Default|SetActorHit _hitactor)
  (Utilities|FlowControl|Sequence
    (:then_0
      (Development|PrintString "collision" false false))
    (:then_1
      (CallFunction|SpawnHitEffect _impactpoint "/Game/Particles/P_Hit.P_Hit"))
    (:then_2
      (CallFunction|DamageEnemy (Variables|Default|GetActorHit))
      (Utilities|FlowControl|Delay 0.01))
    (:then_3
      (Actor|DestroyActor) ; Destroy Projectile when hitting something
    )))

(event EventBeginPlay
  ;[1 1 1] BeginOfPlay
  (Utilities|FlowControl|Sequence
    (:then_1
      (Utilities|FlowControl|Delay 3.0) ; after certain time projectile \ngets destroyed
      (Actor|DestroyActor))))

(fn ConstructionScript)

(fn SpawnHitEffect
  (params (Location :type Vector%20%28by%20ref%29) (Particle :type Particle%20System%20Object%20Reference))
  (Effects|SpawnEmitteratLocation Particle Location))

(fn SetGlowyMaterial
  (params (SourceMaterial :type Material%20Interface%20Object%20Reference))
  (Utilities|FlowControl|Sequence
    (:then_0
      (bind _returnvalue (Rendering|Material|CreateDynamicMaterialInstance (Variables|Default|GetAppearence) 0 SourceMaterial "None" :!class /Script/Engine.PrimitiveComponent))
      (bind _output_get (LocalVariables|SetMID _returnvalue))
      (Rendering|Material|SetMaterial (Variables|Default|GetAppearence) 0 _output_get))
    (:then_1
      (bind _returnvalue_2 (Rendering|Material|GetVectorParameterValue (LocalVariables|GetMID) "LightColor" :!class /Script/Engine.MaterialInstanceDynamic))
      (Rendering|Components|Light|SetLightColor (Variables|Default|GetPointLight) _returnvalue_2 true) ; same color as the material
    )))

(fn DamageEnemy
  (params (HitActor :type Actor%20Object%20Reference%20%28by%20ref%29))
  (bind _asbp_master_enemy (Utilities|Casting|CastToBP_MasterEnemy HitActor))
  (Game|Damage|ApplyDamage _asbp_master_enemy (Variables|Default|GetDamage) 0 0))