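; BP_ShootingSystem provides a Shoot function that fires a projectile with a caller-supplied damage value.
; Shoot runs a camera-channel line trace from start to end, though its result is unused, then spawns the supplied class at the start position with the character's rotation.
; It casts the spawned actor to BP_Projectile and sets its Damage for enemy damage checks.
; The event graph and construction script are empty.
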(event EventBeginPlay)

(event Collision|EventActorBeginOverlap
  (params (OtherActor :type Actor%20Object%20Reference)))

(event EventTick
  (params (DeltaSeconds :type Float%20%28single-precision%29)))

(fn ConstructionScript)

(fn Shoot
  (params (Damage :type Float%20%28single-precision%29) (SpawnedObject :type Actor%20Class%20Reference) (StartPosition :type Vector) (EndPosition :type Vector) (RotationOfCharacter :type Rotator))
  (Utilities|FlowControl|Sequence
    (:then_0
      ;[1 1 1] Calc. Projectie
      (Collision|LineTraceByChannel StartPosition EndPosition "TraceTypeQuery2" false 0 "None" true "(R=1.000000,G=0.000000,B=0.000000,A=1.000000)" "(R=0.000000,G=1.000000,B=0.000000,A=1.000000)" 4.0)
      (bind _returnvalue (Game|SpawnActorfromClass SpawnedObject (Math|Transform|MakeTransform StartPosition RotationOfCharacter) "Undefined" 0 0)) ; Creates Projectile
      ;[1 1 1] Importan for Enemy DMG Check, further details in BP_Projectile
      (bind _asbp_projectile (Utilities|Casting|CastToBP_Projectile _returnvalue))
      (Variables|/Game/Blueprints/Player/BP_Projectile.BP_Projectile_C|SetDamage _asbp_projectile Damage))))