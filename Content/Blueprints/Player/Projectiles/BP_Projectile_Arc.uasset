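; BP_Projectile_Arc is a player projectile that spawns hit effects on contact and hides its mesh at construction.
; Collision overlap prints a debug string, spawns the effect, and destroys after 0.3 seconds only if OverlappedComponent's owner (the projectile's own component, not OtherActor) casts to BP_MasterEnemy.
; A blocking hit spawns the effect and destroys the projectile immediately.
; The DamageEnemy call is disconnected, so no damage is applied here.
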(event OnComponentBeginOverlap(collision)
  (params (OverlappedComponent :type Primitive%20Component%20Object%20Reference) (OtherActor :type Actor%20Object%20Reference) (OtherComp :type Primitive%20Component%20Object%20Reference) (OtherBodyIndex :type Integer) (bFromSweep :type Boolean) (SweepResult :type Hit%20Result%20Structure%20%28by%20ref%29))
  ;[1 1 1] Collision
  (Variables|Default|SetActorHit (Components|GetOwner OverlappedComponent))
  (Utilities|FlowControl|Sequence
    (:then_0
      (Development|PrintString "collision" false false))
    (:then_1
      (CallFunction|SpawnHitEffect (.ImpactPoint (Collision|BreakHitResult SweepResult))))
    (:then_3
      (Utilities|Casting|CastToBP_MasterEnemy (Variables|Default|GetActorHit))
      (Utilities|FlowControl|Delay 0.3)
      (Actor|DestroyActor) ; Destroy Projectile when hitting something
    )))

(event OnComponentHit(collision)
  (params (HitComponent :type Primitive%20Component%20Object%20Reference) (OtherActor :type Actor%20Object%20Reference) (OtherComp :type Primitive%20Component%20Object%20Reference) (NormalImpulse :type Vector :default "0, 0, 0") (Hit :type Hit%20Result%20Structure%20%28by%20ref%29))
  (CallFunction|SpawnHitEffect (.Location (Collision|BreakHitResult Hit)))
  (Actor|DestroyActor) ; Destroy Projectile when hitting something
)

(event EventBeginPlay
  (|CallParentFunction) ; This node is disabled and will not be called.\nDrag off pins to build functionality.
)

(event Collision|EventActorBeginOverlap
  (params (OtherActor :type Actor%20Object%20Reference)))

(fn ConstructionScript
  (|CallParentFunction)
  (Rendering|SetVisibility (Variables|Character|GetMesh) false false))