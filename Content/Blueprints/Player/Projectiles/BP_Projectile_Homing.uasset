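; Player homing projectile that steers toward the nearest living enemy, with its mesh given an invisible material.
; From BeginPlay it re-runs LockOn every 0.2 seconds to set the movement component's homing target.
; FindHomingTarget scans all BP_MasterEnemy actors, skipping those tagged dead.
; The closest distance is never reset between scans, so the target changes only when an enemy beats the smallest distance recorded.
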(event Custom|Lock%20On
  (bind _projectilemovement (Variables|Default|GetProjectileMovement))
  (CallFunction|FindHomingTarget)
  (Utilities|IsValid (Variables|Default|GetClosestEnemy)
    (:Is%20Valid
      (Variables|/Script/Engine.ProjectileMovementComponent|SetHomingTargetComponent _projectilemovement (Actor|GetComponentbyClass (Variables|Default|GetClosestEnemy) "/Script/Engine.SceneComponent"))
      (Variables|/Script/Engine.ProjectileMovementComponent|SetbIsHomingProjectile _projectilemovement true))))

(event EventBeginPlay
  (|CallParentFunction)
  (CallFunction|Lockon :!label _label)
  (Utilities|FlowControl|Delay 0.2)
  (goto _label))

(event Collision|EventActorBeginOverlap
  (params (OtherActor :type Actor%20Object%20Reference)))

(event EventTick
  (params (DeltaSeconds :type Float%20%28single-precision%29)))

(fn ConstructionScript
  (|CallParentFunction)
  (Rendering|Material|SetMaterial (Variables|Character|GetMesh) 0 "/Game/Materials/Misc/M_Invisible.M_Invisible"))

(fn FindHomingTarget
  (bind _outactors (Actor|GetAllActorsOfClass "/Game/Blueprints/Enemy/BP_MasterEnemy.BP_MasterEnemy_C"))
  (for _array_element _outactors
    (if (not (Actor|ActorHasTag _array_element "dead"))
      (bind _output_get (LocalVariables|SetcurrentEnemy _array_element))
      (bind _output_get_2 (LocalVariables|SetcurrentDistaneToEnemy (Math|Float|Absolute(Float) (Math|Vector|Distance(Vector) (Transformation|GetActorLocation _output_get) (Transformation|GetActorLocation)))))
      (if (< _output_get_2 (Variables|Default|GetClosestDistance))
        (Variables|Default|SetClosestDistance (LocalVariables|GetcurrentDistaneToEnemy))
        (Variables|Default|SetClosestEnemy (LocalVariables|GetcurrentEnemy))))))