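; BP_Animal_NPC is a configurable friendly animal NPC whose species, such as deer, cow or fox, is picked through the AnimalToChoose variable.
; The Construction Script maps that choice to an index into FriendlyAnimalsList, swaps in the matching skeletal mesh, then assigns that species' Animation Blueprint.
; Both mappings are hard-coded switches, and the Event Graph holds no active logic, so the Blueprint only handles appearance setup.
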(event EventBeginPlay
  (|CallParentFunction) ; This node is disabled and will not be called.\nDrag off pins to build functionality.
)

(event Collision|EventActorBeginOverlap
  (params (OtherActor :type Actor%20Object%20Reference)))

(event EventTick
  (params (DeltaSeconds :type Float%20%28single-precision%29))
  (|CallParentFunction DeltaSeconds) ; This node is disabled and will not be called.\nDrag off pins to build functionality.
)

(fn ConstructionScript
  (|CallParentFunction)
  (Utilities|FlowControl|Sequence
    (:then_0
      (LocalVariables|SetIndex (CallFunction|GetAnimalIndex (Variables|Default|GetAnimalToChoose))))
    (:then_1
      (Class|SkinnedMeshComponent|SetSkeletalMesh (Variables|Character|GetMesh) (Utilities|Array|Get(acopy) (Utilities|Struct|BreakS_Friendly_Animal (Variables|Default|GetFriendlyAnimalsList)) (LocalVariables|GetIndex)) true)
      (CallFunction|SetAnimationBlueprint (Variables|Default|GetAnimalToChoose)))))

(fn GetAnimalIndex
  (params (Animal :type E_FriendlyAnimals%20Enum :default "NewEnumerator0"))
  (Utilities|FlowControl|Sequence
    (:then_0
      (switch Utilities|FlowControl|Switch|SwitchonE_FriendlyAnimals Animal
        (:NewEnumerator0
          (LocalVariables|SetAnimalIndex 0))
        (:NewEnumerator1
          (LocalVariables|SetAnimalIndex 1))
        (:NewEnumerator2
          (LocalVariables|SetAnimalIndex 2))
        (:NewEnumerator3
          (LocalVariables|SetAnimalIndex 3))
        (:NewEnumerator4
          (LocalVariables|SetAnimalIndex 4))
        (:NewEnumerator5
          (LocalVariables|SetAnimalIndex 5))
        (:NewEnumerator6
          (LocalVariables|SetAnimalIndex 6))))
    (:then_1
      (return (LocalVariables|GetAnimalIndex)))))

(fn SetAnimationBlueprint
  (params (Animal :type E_FriendlyAnimals%20Enum :default "NewEnumerator0"))
  (Utilities|FlowControl|Sequence
    (:then_0
      (switch Utilities|FlowControl|Switch|SwitchonE_FriendlyAnimals Animal
        (:NewEnumerator0
          (LocalVariables|SetAnimationClass "/Game/Models/Wildlife/Deer/AB_Deer.AB_Deer_C"))
        (:NewEnumerator1
          (LocalVariables|SetAnimationClass "/Game/Models/Wildlife/Alpaca/AB_Alpaca.AB_Alpaca_C"))
        (:NewEnumerator2
          (LocalVariables|SetAnimationClass "/Game/Models/Wildlife/Cow/AB_Cow.AB_Cow_C"))
        (:NewEnumerator3
          (LocalVariables|SetAnimationClass "/Game/Models/Wildlife/Fox/AB_Fox.AB_Fox_C"))
        (:NewEnumerator4
          (LocalVariables|SetAnimationClass "/Game/Models/Wildlife/Donkey/AB_Donkey.AB_Donkey_C"))
        (:NewEnumerator5
          (LocalVariables|SetAnimationClass "/Game/Models/Wildlife/Stag/AB_Stag.AB_Stag_C"))
        (:NewEnumerator6
          (LocalVariables|SetAnimationClass "/Game/Models/Wildlife/Bull/AB_Bull.AB_Bull_C"))))
    (:then_1
      (Class|SkeletalMeshComponent|SetAnimClass (Variables|Character|GetMesh) (LocalVariables|GetAnimationClass)))))