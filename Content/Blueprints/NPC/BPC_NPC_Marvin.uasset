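; Marvin NPC Blueprint that gives quest-aware dialogue when the player talks to it.
; OnTalkto asks the player's QuestManager for the QUEST_DEMO01 quest and checks whether goal index 2 is among its current goals.
; If so, it shows a short timed greeting message; otherwise it falls back to the parent class's talk behavior.
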(event EventBeginPlay
  (|CallParentFunction) ; This node is disabled and will not be called.\nDrag off pins to build functionality.
)

(event Collision|EventActorBeginOverlap
  (params (OtherActor :type Actor%20Object%20Reference)))

(event EventTick
  (params (DeltaSeconds :type Float%20%28single-precision%29)))

(event EventOnTalkto
  (params (Player :type BP%20Player%20Object%20Reference))
  (bind _questmanager (Variables|/Game/Blueprints/Player/BP_Player.BP_Player_C|GetQuestManager Player))
  (bind (_out _questactor) (Default|HasCurrentQuest _questmanager "/Game/Blueprints/Actors/QuestSystem/QuestActors/QUEST_DEMO01.QUEST_DEMO01_C"))
  (if _out
    (if (Utilities|Array|ContainsItem (Variables|/Game/Blueprints/Actors/QuestSystem/QuestActors/BP_MasterQuest.BP_MasterQuest_C|GetCurrentGoalIndices _questactor) 2)
      (CallFunction|ShowMessage "Ah, now we can talk. How are you?" 5.0 Player)
      (else
        (|CallParentFunction Player :!label _label)))
    (else
      (goto _label))))

(fn ConstructionScript
  (|CallParentFunction))