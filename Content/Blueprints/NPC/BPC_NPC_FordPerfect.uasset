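; Ford Perfect NPC, a child Blueprint that hands out a single quest once the player has earned enough prestige in a required area.
; A prestige-gain event checks the threshold, then enables the quest, swaps the NPC dot for a question mark and sets the interaction prompt.
; Interacting adds and starts the quest through the player's QuestManager, restores the dot and changes the default message.
; All other interactions fall back to the parent behavior.
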(event EventBeginPlay
  (|CallParentFunction) ; This node is disabled and will not be called.\nDrag off pins to build functionality.
)

(event Collision|EventActorBeginOverlap
  (params (OtherActor :type Actor%20Object%20Reference)))

(event EventTick
  (params (DeltaSeconds :type Float%20%28single-precision%29)))

(event EventOnInteractwith
  (params (Player :type BP%20Player%20Object%20Reference))
  (if (and (Variables|Default|GetCanGiveQuest) (not (Variables|Default|GetHasGivenQuest)))
    (Default|AddNewQuest (Variables|/Game/Blueprints/Player/BP_Player.BP_Player_C|GetQuestManager Player) (Variables|Default|GetQuestToGive) true)
    (Variables|Default|SetHasGivenQuest true)
    (Variables|Default|SetDefaultMessage "Now I like you. Mind to keep your towel with you. Always!")
    (Rendering|SetVisibility (Variables|Default|GetQuestionMark) false false)
    (Rendering|SetVisibility (Variables|Default|GetNPCDot) true false)
    (else
      (|CallParentFunction Player))))

(event EventOnPlayerGainPP
  (params (Player :type BP%20Player%20Object%20Reference))
  (bind _requiredpp (Variables|Default|GetRequiredPP))
  (bind (_area _prestige) (Utilities|Struct|BreakS_AreaPrestige _requiredpp))
  (if (Math|Boolean|ANDBoolean (>= (Default|GetPrestigebyArea Player _area) _prestige) (not (Variables|Default|GetCanGiveQuest)) (not (Variables|Default|GetHasGivenQuest)))
    (Variables|Default|SetCanGiveQuest true)
    (Rendering|SetVisibility (Variables|Default|GetNPCDot) false false)
    (Rendering|SetVisibility (Variables|Default|GetQuestionMark) true false)
    (CallFunction|SetInteractionText "Press [E] to interact" (Variables|Default|GetInteractionWidget) (Variables|Default|GetQuestToGive))))

(fn ConstructionScript
  (|CallParentFunction))