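; Master NPC character that can give the player a quest or show a timed dialogue message on interaction.
; Quest markers and the interaction prompt depend on HasQuest; interacting adds the quest to the player's QuestManager, and talking reports the NPC to it for quest tracking.
; An overlap radius and spawn location feed the AI blackboard.
; Tick-updated movement stats are exposed through interface getters, and the head follows the body via master pose.
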(event OnComponentBeginOverlap(InteractionRadius)
  (params (OverlappedComponent :type Primitive%20Component%20Object%20Reference) (OtherActor :type Actor%20Object%20Reference) (OtherComp :type Primitive%20Component%20Object%20Reference) (OtherBodyIndex :type Integer) (bFromSweep :type Boolean) (SweepResult :type Hit%20Result%20Structure%20%28by%20ref%29))
  (AI|Components|Blackboard|SetValueasBool (Variables|Default|GetBlackboard) (Variables|Default|GetInInteractionDistance) true))

(event OnComponentEndOverlap(InteractionRadius)
  (params (OverlappedComponent :type Primitive%20Component%20Object%20Reference) (OtherActor :type Actor%20Object%20Reference) (OtherComp :type Primitive%20Component%20Object%20Reference) (OtherBodyIndex :type Integer))
  (AI|Components|Blackboard|SetValueasBool (Variables|Default|GetBlackboard) (Variables|Default|GetInInteractionDistance) false))

(event Custom|OnPlayerLevelUp
  (params (NewLevel :type Integer)))

(event Custom|OnPlayerGainPP
  (params (Player :type BP%20Player%20Object%20Reference)))

(event EventTick
  (params (DeltaSeconds :type Float%20%28single-precision%29))
  (CallFunction|UpdateMovementStats))

(event EventBeginPlay
  (bind _self self)
  (Utilities|FlowControl|Sequence
    (:then_0
      (CallFunction|BeginOfPlay)
      (Actor|SetOwner (Game|GetPlayerCharacter 0))
      (if (Utilities|IsValidClass (Variables|Default|GetHasQuest))
        (Rendering|SetVisibility (Variables|Default|GetQuestionMark) true false) ; set question mark sprite, if npc has quest
        (else
          (Rendering|SetVisibility (Variables|Default|GetNPCDot) true false))))
    (:then_1
      (bind _aswbp_interaction (Utilities|Casting|CastToWBP_Interaction (UserInterface|GetUserWidgetObject (Variables|Default|GetInteractionWidget))))
      (Rendering|Components|TextRender|SetText (Variables|/Game/Blueprints/UI/NPC/WBP_Interaction.WBP_Interaction_C|GetName _aswbp_interaction) (Variables|Default|GetName)) ; set npc name
      (CallFunction|SetInteractionText "Press [E] to interact" (Variables|Default|GetInteractionWidget) (Variables|Default|GetHasQuest))
      (Variables|Default|SetBlackboard (AI|GetBlackboard 0)))
    (:then_2
      (AI|Components|Blackboard|SetValueasVector (Variables|/Script/AIModule.AIController|GetBlackboard (AI|GetAIController _self)) (Variables|Default|GetMapLocation) (Transformation|GetActorLocation _self)))))

(event EventOnInteractwith
  (params (Player :type BP%20Player%20Object%20Reference))
  (bind _questmanager (Variables|/Game/Blueprints/Player/BP_Player.BP_Player_C|GetQuestManager Player))
  (bind _hasquest (Variables|Default|GetHasQuest))
  ;[1 1 1] On interaction with NPC, Quest Dialogue, Add Quest
  (if (Utilities|IsValidClass _hasquest)
    (if (Utilities|Array|ContainsItem (Variables|/Game/Blueprints/Actors/QuestSystem/BP_QuestManager.BP_QuestManager_C|GetAllQuestClasses _questmanager) _hasquest)
      (CallFunction|OnTalkto Player :!label _label)
      (else
        (Default|AddNewQuest _questmanager (Variables|Default|GetHasQuest) false)
        (Rendering|SetVisibility (Variables|Default|GetQuestionMark) false false)
        (Rendering|SetVisibility (Variables|Default|GetNPCDot) true false)))
    (else
      (goto _label))))

(event Custom|OnTalkTo
  (params (Player :type BP%20Player%20Object%20Reference))
  ;[1 1 1] On Talk To
  (CallFunction|ShowMessage (Variables|Default|GetDefaultMessage) (Variables|Default|GetDefaultDuration) Player))

(event Custom|ShowMessage
  (params (Message :type Text) (Duration :type Float%20%28single-precision%29) (Player :type BP%20Player%20Object%20Reference))
  (bind _hud (Variables|/Game/Blueprints/Player/BP_Player.BP_Player_C|GetHUD Player))
  (bind _wbp_dialogemessage (Variables|/Game/Blueprints/UI/HUD/WBP_Main.WBP_Main_C|GetWBP_DialogeMessage _hud))
  ;[1 1 1] Event Show Message
  (if (Variables|Default|GetCanTalkWith)
    (Variables|Default|SetCanTalkWith false)
    (Rendering|Components|TextRender|SetText (Variables|/Game/Blueprints/UI/NPC/WBP_DialogeMessage.WBP_DialogeMessage_C|GetName _wbp_dialogemessage) (Variables|Default|GetName))
    (Rendering|Components|TextRender|SetText (Variables|/Game/Blueprints/UI/NPC/WBP_DialogeMessage.WBP_DialogeMessage_C|GetMessage _wbp_dialogemessage) Message)
    (Widget|SetVisibility _wbp_dialogemessage "Visible")
    (Default|OnTalkedtoNPC (Variables|/Game/Blueprints/Player/BP_Player.BP_Player_C|GetQuestManager Player) (Utilities|GetClass self) (Variables|Default|GetNPC_ID))
    (Utilities|FlowControl|Delay Duration)
    (Widget|SetVisibility _wbp_dialogemessage "Hidden")
    (Variables|Default|SetCanTalkWith true)))

(event Custom|OnOwnQuestCancelled
  (params (Class :type BP%20Master%20Quest%20Class%20Reference))
  (Rendering|SetVisibility (Variables|Default|GetQuestionMark) true false))

(event Custom|UpdateMovementStats
  (Variables|Movement|SetSpeed (CallFunction|GetCurrentSpeed))
  (Variables|Movement|SetDirection (CallFunction|GetCurrentDirection))
  (Variables|Movement|SetisStandingStill? (Math|Float|NearlyEqual(Float) (Variables|Movement|GetSpeed) 0.0 0.01)))

(fn ConstructionScript
  (Class|SkinnedMeshComponent|SetMasterPoseComponent (Variables|Default|GetHead) (Variables|Character|GetMesh) false))

(fn SetInteractionText
  (params (Text :type Text) (Widget :type Widget%20Component%20Object%20Reference) (LocalHasQuest :type BP%20Master%20Quest%20Class%20Reference))
  (bind _aswbp_interaction (Utilities|Casting|CastToWBP_Interaction (UserInterface|GetUserWidgetObject Widget))
    (:then
      (if (Utilities|IsValidClass LocalHasQuest)
        (Rendering|Components|TextRender|SetText (Variables|/Game/Blueprints/UI/NPC/WBP_Interaction.WBP_Interaction_C|GetInteractionText _aswbp_interaction) Text) ; if npc has quest, add interaction text
      )
      (return))
    (:CastFailed
      (return))))

(fn GetCurrentSpeed
  (return (Math|Float|MapRangeClamped (Math|Vector|VectorLength (Transformation|GetVelocity)) 0.0 (Class|MovementComponent|GetMaxSpeed (Variables|Character|GetCharacterMovement)) 0.0 1.0)))

(fn GetCurrentDirection
  (bind _returnvalue (Transformation|GetVelocity))
  (bind (_x _y) (Math|Vector|BreakVector _returnvalue))
  (return (Class|KismetMathLibrary|ClampAxis (Class|AnimInstance|CalculateDirection (Variables|Ref|GetMainAnimInstance) (Math|Vector|MakeVector _x _y 0.0) (Transformation|GetActorRotation)))))

(fn BeginOfPlay
  (bind _mesh (Variables|Character|GetMesh))
  (bind _returnvalue (Components|SkeletalMesh|GetAnimInstance _mesh))
  (Utilities|FlowControl|Sequence
    (:then_0
      (Utilities|IsValid _returnvalue
        (:Is%20Valid
          (Variables|Ref|SetMainAnimInstance _returnvalue))))
    (:then_1
      (Class|SkinnedMeshComponent|SetMasterPoseComponent (Variables|Default|GetHead) _mesh false))))

(fn BPIGetMovementStates
  (return (not (Variables|Movement|GetisStandingStill?)) false false false (AI|Components|NavMovement|IsFalling (Variables|Character|GetCharacterMovement)) false))

(fn BPIGetMovementStats
  (return (Transformation|GetVelocity) "0, 0, 0" (Variables|Movement|GetSpeed) (Variables|Movement|GetDirection) 0.0))