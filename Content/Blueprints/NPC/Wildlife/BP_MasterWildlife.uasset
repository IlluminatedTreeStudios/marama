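; Master wildlife Blueprint that configures a neutral animal from its Type enum.
; The enum name keys a DT_Neutral_Wildlife row supplying mesh and anim class at construction, and animations at BeginPlay.
; Tick measures velocity and derives moving, walking and sprinting flags using tolerance bands around speeds from the fixed Wildlife_1 row of DT_MovementSpeed.
; Interface getters expose these states and stats, with crouch, jump, air and turn values stubbed.
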(event Custom|updateMovementValues
  (bind _output_get (Variables|Movement-Stats|SetSpeed (Math|Vector|VectorLength (Transformation|GetVelocity))))
  (Development|PrintString (Utilities|String|ToString(Float) _output_get) false false "(R=0.000000,G=0.660000,B=1.000000,A=1.000000)" 0.0)
  (CallFunction|SetMovementStates))

(event EventBeginPlay
  (Character-Mesh|SetAnimations)
  (bind _returnvalue (Utilities|GetDataTableRow "/Game/Blueprints/DataTables/Movement/DT_MovementSpeed.DT_MovementSpeed" "Wildlife_1")
    (:then
      (Variables|Movement-Stats|SetMovementSpeedValues _returnvalue))))

(event Collision|EventActorBeginOverlap
  (params (OtherActor :type Actor%20Object%20Reference)))

(event EventTick
  (params (DeltaSeconds :type Float%20%28single-precision%29))
  (CallFunction|UpdateMovementValues))

(fn ConstructionScript
  (Character-Mesh|SetMesh)
  (Character-Mesh|SetAnimClass))

(fn GetAnimalInformation
  (params (Type :type E_FriendlyAnimals%20Enum :default "NewEnumerator0"))
  (Utilities|FlowControl|Sequence
    (:then_0
      (LocalVariables|SetAnimalName (Utilities|String|StringToName (Utilities|String|EnumtoString Type))))
    (:then_1
      (bind _returnvalue (Utilities|GetDataTableRow "/Game/Blueprints/DataTables/DT_Neutral_Wildlife.DT_Neutral_Wildlife" (LocalVariables|GetAnimalName))
        (:then
          (return _returnvalue))))))

(fn SetMesh
  (Utilities|FlowControl|Sequence
    (:then_0
      (LocalVariables|SetNewMesh (.Mesh (Utilities|Struct|BreakS_SkeletalMeshAndAnimations (Character-Mesh|GetAnimalInformation (Variables|Default|GetType))))))
    (:then_1
      (Class|SkinnedMeshComponent|SetSkeletalMesh (Variables|Character|GetMesh) (LocalVariables|GetNewMesh) true))))

(fn SetAnimations
  (Variables|Animation|SetAnimations (.Animations (Utilities|Struct|BreakS_SkeletalMeshAndAnimations (Character-Mesh|GetAnimalInformation (Variables|Default|GetType))))))

(fn SetAnimClass
  (Class|SkeletalMeshComponent|SetAnimClass (Variables|Character|GetMesh) (.AnimationBP (Utilities|Struct|BreakS_SkeletalMeshAndAnimations (Character-Mesh|GetAnimalInformation (Variables|Default|GetType))))))

(fn SetMovementStates
  (bind _movementspeedvalues (Variables|Movement-Stats|GetMovementSpeedValues))
  (bind (_walkspeed _sprintspeed) (Utilities|Struct|BreakS_MovementSettings_Speed (.standard _movementspeedvalues)))
  (Utilities|FlowControl|Sequence
    (:then_0
      (Variables|Movement-State|SetisMoving (not (Math|Float|NearlyEqual(Float) (Variables|Movement-Stats|GetSpeed) 0.0 1.0))))
    (:then_1
      (Variables|Movement-State|SetIsWalking (Math|Float|NearlyEqual(Float) (Variables|Movement-Stats|GetSpeed) _walkspeed (/ _walkspeed 2.0))))
    (:then_2
      (Variables|Movement-State|SetIsSprinting (Math|Float|NearlyEqual(Float) (Variables|Movement-Stats|GetSpeed) _sprintspeed (/ _sprintspeed 2.0))))))

(fn BPIGetMovementStates
  (return (Variables|Movement-State|GetisMoving) false (Variables|Movement-State|GetIsSprinting) false false (Variables|Movement-State|GetIsWalking)))

(fn BPIGetMovementStats
  (return (Transformation|GetVelocity) "0, 0, 0" (Variables|Movement-Stats|GetSpeed) 0.0 0.0))