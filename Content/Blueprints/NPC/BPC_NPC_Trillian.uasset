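; Trillian NPC Blueprint that offers a quest, involving a search for a towel, once the player reaches a required level.
; On level-up it unlocks the quest, swaps the NPC dot for a question mark and updates the interaction prompt.
; Interacting then adds and starts the quest through the player's QuestManager, changes the default message and restores the dot.
; All other interactions fall through to the parent NPC behavior.
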(event EventBeginPlay
  (|CallParentFunction) ; This node is disabled and will not be called.\nDrag off pins to build functionality.
)

(event Collision|EventActorBeginOverlap
  (params (OtherActor :type Actor%20Object%20Reference)))

(event EventTick
  (params (DeltaSeconds :type Float%20%28single-precision%29)))

(event EventOnPlayerLevelUp
  (params (NewLevel :type Integer))
  (if (Math|Boolean|ANDBoolean (>= NewLevel (Variables|Default|GetRequiredLevel)) (not (Variables|Default|GetCanGiveQuest)) (not (Variables|Default|GetHasGivenQuest)))
    (Variables|Default|SetCanGiveQuest true)
    (Rendering|SetVisibility (Variables|Default|GetNPCDot) false false)
    (Rendering|SetVisibility (Variables|Default|GetQuestionMark) true false)
    (CallFunction|SetInteractionText "Press [E] to interact" (Variables|Default|GetInteractionWidget) (Variables|Default|GetQuestToGive))))

(event EventOnInteractwith
  (params (Player :type BP%20Player%20Object%20Reference))
  (if (and (Variables|Default|GetCanGiveQuest) (not (Variables|Default|GetHasGivenQuest)))
    (Default|AddNewQuest (Variables|/Game/Blueprints/Player/BP_Player.BP_Player_C|GetQuestManager Player) (Variables|Default|GetQuestToGive) true)
    (Variables|Default|SetHasGivenQuest true)
    (Variables|Default|SetDefaultMessage "Now you are strong enough. Can you help me finding my towel?")
    (Rendering|SetVisibility (Variables|Default|GetQuestionMark) false false)
    (Rendering|SetVisibility (Variables|Default|GetNPCDot) true false)
    (else
      (|CallParentFunction Player))))

(fn ConstructionScript
  (|CallParentFunction))