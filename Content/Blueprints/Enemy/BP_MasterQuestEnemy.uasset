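; Master quest enemy Blueprint that overrides its parent's melee hit area placement and attack glow effect for attacks using both hands.
; Construction assigns the AttackEffect asset to left and right hand Niagara glow components.
; SetHitAreaLocation replaces the parent logic, attaching HitArea to the left or right hand socket for the first or second combo attack.
; The darkness effect toggle calls the parent with a fixed false, then activates or deactivates both glows.
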(fn ConstructionScript
  (|CallParentFunction)
  (Class|NiagaraComponent|SetAsset (Variables|Default|GetNS_LeftHand_Glow) (Variables|Default|GetAttackEffect) false))

(fn SetHitAreaLocation
  (if (== (Variables|Default|GetAttackComboIndex) 0) ; 1st Anim
    (Transformation|AttachComponentToComponent (Variables|Default|GetHitArea) (Variables|Character|GetMesh) "LH_S" "KeepRelative" "KeepRelative" "KeepRelative" true)
    (elif (== (Variables|Default|GetAttackComboIndex) 1) ; 2nd Anim
      (Transformation|AttachComponentToComponent (Variables|Default|GetHitArea) (Variables|Character|GetMesh) "RH_S" "KeepRelative" "KeepRelative" "KeepRelative" true))))

(fn AttackToggleDarknessEffect
  (params (On/Off? :type Boolean))
  (bind _ns_lefthand_glow (Variables|Default|GetNS_LeftHand_Glow))
  (|CallParentFunction false)
  (if On/Off?
    (Components|Activation|Activate _ns_lefthand_glow false)
    (else
      (Components|Activation|Deactivate _ns_lefthand_glow))))