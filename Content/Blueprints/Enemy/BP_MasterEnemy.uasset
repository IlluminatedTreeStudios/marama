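; Base enemy character Blueprint handling health bar, patrol and chase speeds, melee combo attacks, damage and death, with hooks for derived enemies.
; The AI controller starts attacks, cycling montages while anim notifies trigger sphere traces against the player.
; Damage ignores other enemies, and death awards XP, notifies quests and plays an optional darkness effect.
; Respawning goes through a respawn actor, linked to or spawned at its associated glowing tree.
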(event Custom|setRespawner
  ;[1 1 1] Respawner
  (Utilities|IsValid (Variables|Respawn|GetRespawnActor)
    (:Is%20Valid
      (if (Utilities|Enum|Equal(Enum) "NewEnumerator5" (Variables|Respawn|GetRespawnAssociatedToTree))
        (Variables|/Game/Blueprints/Enemy/BP_EnemyRespawn.BP_EnemyRespawn_C|SetRespawnAssociatedTree (Variables|Respawn|GetRespawnActor) (Variables|Respawn|GetRespawnAssociatedToTree))
        (else
          (bind _outactors (Actor|GetAllActorsOfClass "/Game/Blueprints/Actors/GlowingTree/BP_GlowingTree_Master.BP_GlowingTree_Master_C" :!label _label)) ; Tree Associated
          (for _array_element _outactors
            (if (Utilities|Enum|Equal(Enum) (Variables|Respawn|GetRespawnAssociatedToTree) (Variables|/Game/Blueprints/Actors/GlowingTree/BP_GlowingTree_Master.BP_GlowingTree_Master_C|GetRespawn%20Point _array_element)) ; which tree is associated?
              (Utilities|FlowControl|Sequence
                (:then_0
                  (Utilities|IsValid (Variables|Respawn|GetRespawnActor) ; check if respawn is directly\nat tree or set manually\n-> if manually set then \nrespawn actor is not none
                    (:Is%20Valid
                      (Variables|/Game/Blueprints/Enemy/BP_EnemyRespawn.BP_EnemyRespawn_C|SetatTreeRespawn? (Variables|Respawn|GetRespawnActor) false))
                    (:Is%20Not%20Valid
                      (bind _returnvalue (Game|SpawnActorfromClass "/Game/Blueprints/Enemy/BP_EnemyRespawn.BP_EnemyRespawn_C" (Math|Transform|MakeTransform (Transformation|GetActorLocation _array_element) "0, 0, 0" "1,1,1") "Undefined" 0 0)) ; creates respawn actor at tree location
                      (bind _output_get (Variables|Respawn|SetRespawnActor _returnvalue))
                      (Variables|/Game/Blueprints/Enemy/BP_EnemyRespawn.BP_EnemyRespawn_C|SetatTreeRespawn? _output_get true))))
                (:then_1
                  (Variables|/Game/Blueprints/Enemy/BP_EnemyRespawn.BP_EnemyRespawn_C|SetTree (Variables|Respawn|GetRespawnActor) _array_element)
                  (Variables|/Game/Blueprints/Enemy/BP_EnemyRespawn.BP_EnemyRespawn_C|SetRespawnAssociatedTree (Variables|Respawn|GetRespawnActor) (Variables|Respawn|GetRespawnAssociatedToTree)))))))))
    (:Is%20Not%20Valid
      (goto _label))))

(event EventBeginPlay
  (bind _returnvalue (Game|GetPlayerCharacter 0))
  (bind _self self)
  ;[1 1 1] BeginPlay
  (Utilities|FlowControl|Sequence
    (:then_0
      (Actor|SetOwner _returnvalue)
      (Rendering|SetVisibility (Variables|UI|GetEnemyDot) true false))
    (:then_1
      (bind _asbp_player (Utilities|Casting|CastToBP_Player _returnvalue))
      (Variables|Reference|SetTarget%28Player%29 _asbp_player)
      (Variables|Stats|SetCurrentHP (Variables|Stats|GetMaxHP))
      (UI|SetUpWidget))
    (:then_2
      (AI|Components|Blackboard|SetValueasVector (Variables|/Script/AIModule.AIController|GetBlackboard (AI|GetAIController _self)) (Variables|Reference|GetMapLocation) (Transformation|GetActorLocation _self)))
    (:then_3
      (CallFunction|SetRespawner))))

(event Custom|Walk
  ;[1 1 1] Standard Movement
  (Movement|UpdateWalkSpeed (Variables|Stats|GetPatrolSpeed))
  (Variables|State|SetIsRunning false))

(event Custom|Run
  ;[1 1 1] Standard Movement
  (Movement|UpdateWalkSpeed (Variables|Stats|GetChaseSpeed))
  (Variables|State|SetIsRunning true))

(event OnComponentBeginOverlap(CapsuleComponent)
  (params (OverlappedComponent :type Primitive%20Component%20Object%20Reference) (OtherActor :type Actor%20Object%20Reference) (OtherComp :type Primitive%20Component%20Object%20Reference) (OtherBodyIndex :type Integer) (bFromSweep :type Boolean) (SweepResult :type Hit%20Result%20Structure%20%28by%20ref%29))
  (if (not (Actor|ActorHasTag "dead"))
    (bind _asbp_projectile_arc (Utilities|Casting|CastToBP_Projectile_Arc (Components|GetOwner OtherComp)))
    (Development|PrintString "OVERLAP COLLIDE")
    (Game|Damage|ApplyDamage self (Variables|/Game/Blueprints/Player/Projectiles/BP_Projectile.BP_Projectile_C|GetDamage _asbp_projectile_arc) 0 0 "/Game/Blueprints/DmgTypes/Dmg_Light.Dmg_Light_C")))

(event Custom|Hit
  ;[1 1 1] Getting Hit
  (Components|Movement|StopMovementImmediately (Variables|Character|GetCharacterMovement))
  (Animation|Montage|PlayMontage (Variables|Character|GetMesh) (Variables|Animation|GetGettingHitAnimationToPlay)))

(event Custom|Death
  ;[1 1 1] DEATH
  (Utilities|FlowControl|DoOnce false
    (:Completed
      (Utilities|FlowControl|Sequence
        (:then_0
          ;;[1 1 1] earned XP from defeating enemy
          (Default|AddXpPoints (Variables|Reference|GetTarget%28Player%29) (Variables|Stats|GetXPtoEarn))
          ;;[1 1 1] Misc.
          (Default|KilledEnemy (Variables|Reference|GetTarget%28Player%29) (Variables|Stats|GetMaxHP))
          (Components|Activation|Deactivate (Variables|Effects|GetPS_DarknessAura))
          (Utilities|Array|Add (Variables|Actor|GetTags) "dead") ; so homing missiles dont\naim at dead enemies
        )
        (:then_1
          ;;[1 1 1] check if quest enemy
          (bind _asbp_player (Utilities|Casting|CastToBP_Player (Game|GetPlayerCharacter 0)))
          (for _array_element (Variables|/Game/Blueprints/Actors/QuestSystem/BPC_QuestLog.BPC_QuestLog_C|GetQuests (Variables|/Game/Blueprints/Player/BP_Player.BP_Player_C|GetBPC_QuestLog _asbp_player))
            (Default|CallKilledEnemy _array_element self)))
        (:then_2
          ;;[1 1 1] destroy health bar
          (Components|DestroyComponent (Variables|UI|GetEnemyHealthWidget)))
        (:then_3
          ;;[1 1 1] prep for destruction
          (Components|Movement|StopMovementImmediately (Variables|Character|GetCharacterMovement))
          (Class|Pawn|DetachfromControllerPendingDestroy)
          (Rendering|SetVisibility (Variables|UI|GetEnemyDot) false false))
        (:then_4
          ;;[1 1 1] respawning (can be disabled by removing link)
          (CallFunction|Respawn))
        (:then_5
          ;;[1 1 1] Death Animation
          (Animation|Montage|PlayMontage (Variables|Character|GetMesh) (Variables|Animation|GetDeathAnimationToPlay)
            (:OnBlendOut
              _)
            (:OnNotifyEnd
              _))
          (if (Variables|Type|GetDarknessCorruption?)
            (CallFunction|DeathDarknessEffect)
            (else
              (Actor|DestroyActor))))))))

(event Custom|Respawn
  (bind _respawnactor (Variables|Respawn|GetRespawnActor))
  ;[1 1 1] DEATH
  ;;[1 1 1] respawning (can be disabled by removing link)
  (Utilities|IsValid _respawnactor
    (:Is%20Valid
      (Default|RespawnEnemy _respawnactor (Utilities|Struct|MakeS_EnemyRespawn (Variables|Respawn|GetRespawnTime) (Utilities|GetClass self))))))

(event Custom|Death_DarknessEffect
  (Rendering|SetVisibility (Variables|Character|GetMesh) false true)
  (Collision|SetCollisionResponsetoAllChannels (Variables|Collision|GetCapsuleComponent) "ECR_Ignore")
  (Niagara|SpawnSystemAttached (Utilities|Array|Get(acopy) (Variables|Effects|GetDeathParticles)) (Variables|Character|GetMesh) "Root" "0, 0, 0" "0, 0, 0" "KeepRelativeOffset" true)
  (Niagara|SpawnSystematLocation (Utilities|Array|Get(acopy) (Variables|Effects|GetDeathParticles) 1) (Transformation|GetActorLocation))
  (Utilities|FlowControl|Delay 5.0)
  (Actor|DestroyActor))

(event Game|Damage|EventAnyDamage
  (params (Damage :type Float%20%28single-precision%29) (DamageType :type Damage%20Type%20Object%20Reference) (InstigatedBy :type Controller%20Object%20Reference) (DamageCauser :type Actor%20Object%20Reference))
  ;[1 1 1] Takes Damage
  (bind _output_get (Variables|Combat|SetDamageCauser DamageCauser))
  (Utilities|Casting|CastToBP_MasterEnemy _output_get ; Check for friendly fire
    (:CastFailed
      (Combat|TakeDamage Damage)
      (Components|Activation|Activate (Variables|Effects|GetPS_GettingHit) true)
      (if (Variables|State|GetIsDead)
        (CallFunction|Death)
        (else
          (CallFunction|Hit))))))

(event Custom|StartAttack
  ;[1 1 1] Start Of Attack
  (Variables|State|SetIsAttacking true)
  (CallFunction|PlayAttackAnim))

(event Custom|PlayAttackAnim
  (Utilities|FlowControl|DoOnce false ; Ensures Animaiton is Played out\nuntil moment of ResetAttack\nlike chain into next attack
    (:Completed
      (Utilities|FlowControl|Sequence
        (:then_0
          (Animation|GetAttackAnimations (Variables|Animation|GetAttackComboAnims)))
        (:then_1
          (Mesh|SetHitAreaLocation) ; overriden by derived BPs
          (Variables|Combat|SetPlayerHasBeenHit false)
          (Variables|/Script/Engine.CharacterMovementComponent|SetbOrientRotationToMovement (Variables|Character|GetCharacterMovement) false))
        (:then_2
          (bind _notifyname (Animation|Montage|PlayMontage (Variables|Character|GetMesh) (Variables|Animation|GetAttackAnimationToPlay))
            (:then
              (Math|Integer|IncrementInt (Variables|Animation|GetAttackComboIndex)))
            (:OnCompleted
              (Utilities|FlowControl|Sequence :!label _label
                (:then_0
                  (Variables|Combat|SetPlayerHasBeenHit false)
                  (Variables|State|SetIsAttacking false))
                (:then_1
                  (Variables|/Script/Engine.CharacterMovementComponent|SetbOrientRotationToMovement (Variables|Character|GetCharacterMovement) false))
                (:then_2
                  (CallFunction|ResetAttack))))
            (:OnBlendOut
              (goto _label))
            (:OnInterrupted
              (goto _label))
            (:OnNotifyBegin
              (switch name _notifyname
                (:AttackEffect
                  (if (Variables|Type|GetDarknessCorruption?)
                    (CallFunction|AttackToggleDarknessEffect true)))))
            (:OnNotifyEnd
              (switch name _notifyname
                (:AttackEffect
                  (if (Variables|Type|GetDarknessCorruption?)
                    (CallFunction|AttackToggleDarknessEffect false)))))))))))

(event Custom|ResetAttack
  (Utilities|FlowControl|DoOnce false) ; enters at Reset
)

(event Custom|Attack_ToggleDarknessEffect
  (params (On/Off? :type Boolean)))

(event Custom|AttackHit
  (bind _hitmesh (Variables|Default|GetHitMesh))
  (bind _returnvalue (Transformation|GetSocketLocation _hitmesh "Center"))
  ;[1 1 1] Uses Tracers on the socket to detect hit (big slow swing)
  (if (not (Variables|Combat|GetPlayerHasBeenHit))
    (Combat|CheckPlayerHit (Variables|Stats|GetAttackingDamage) _returnvalue _returnvalue (Variables|Combat|GetHitSphereRadius))))

(fn ConstructionScript
  (Rendering|SetVisibility (Variables|Combat|GetHitArea) false true)
  (Class|SkinnedMeshComponent|SetMasterPoseComponent (Variables|Mesh|GetHead) (Variables|Character|GetMesh) false))

(fn UpdateWalkSpeed
  (params (NewWalkSpeed :type Float%20%28single-precision%29))
  (Variables|/Script/Engine.CharacterMovementComponent|SetMaxWalkSpeed (Variables|Character|GetCharacterMovement) NewWalkSpeed))

(fn TakeDamage
  (params (DamageToTake :type Float%20%28single-precision%29))
  (LocalVariables|SetDamage DamageToTake)
  (bind _output_get (Variables|Stats|SetCurrentHP (- (Variables|Stats|GetCurrentHP) (LocalVariables|GetDamage))))
  (if (<= _output_get 0.0)
    (Variables|State|SetIsDead true)
    (Development|PrintString "Is DEAD" true false "(R=1.000000,G=0.000000,B=0.000000,A=1.000000)") ; Replace by saving stats and restart Level
    (else
      (Development|PrintString (Utilities|String|ToString(Float) (Variables|Stats|GetCurrentHP)) false false "(R=1.000000,G=0.820607,B=0.000000,A=1.000000)")))
  (UI|UpdateWidgetHealth))

(fn CheckPlayerHit
  (params (Damage :type Float%20%28single-precision%29) (Start :type Vector%20%28by%20ref%29) (End :type Vector%20%28by%20ref%29) (HitSphereRadius :type Float%20%28single-precision%29))
  (LocalVariables|SetDmg Damage)
  (bind (_outhit _returnvalue) (Collision|SphereTraceForObjects Start End HitSphereRadius (Utilities|Array|MakeArray "ObjectTypeQuery7") false 0 "None" true "(R=1.000000,G=0.000000,B=0.000000,A=1.000000)" "(R=0.000000,G=1.000000,B=0.000000,A=1.000000)" 1.0))
  (if _returnvalue
    (Variables|Combat|SetPlayerHasBeenHit true)
    (Game|Damage|ApplyDamage (.HitActor (Collision|BreakHitResult _outhit)) (LocalVariables|GetDmg) 0 0 (Variables|Combat|GetDamageType))))

(fn GetAttackSockets
  (params (SocketStart :type Name :default "LeftForeArmSocket") (SocketEnd :type Name :default "LeftHandSocket"))
  (bind _mesh (Variables|Character|GetMesh))
  (return (Transformation|GetSocketLocation _mesh SocketStart) (Transformation|GetSocketLocation _mesh SocketEnd)))

(fn UpdateWidgetHealth
  (Progress|SetPercent (Variables|/Game/Blueprints/UI/Enemy/WBP_Enemy.WBP_Enemy_C|GetHealthBar (Variables|Reference|GetEnemyWidget)) (/ (Variables|Stats|GetCurrentHP) (Variables|Stats|GetMaxHP)))
  (return))

(fn SetUpWidget
  (bind _aswbp_enemy (Utilities|Casting|CastToWBP_Enemy (UserInterface|GetUserWidgetObject (Variables|UI|GetEnemyHealthWidget)))
    (:then
      (bind _output_get (Variables|Reference|SetEnemyWidget _aswbp_enemy))
      (Rendering|Components|TextRender|SetText (Variables|/Game/Blueprints/UI/Enemy/WBP_Enemy.WBP_Enemy_C|GetEnemyName _output_get) (Variables|UI|GetNameOfEnemy))
      (UI|UpdateWidgetHealth)
      (Rendering|SetVisibility (Variables|UI|GetEnemyHealthWidget) true false)
      (return))
    (:CastFailed
      (return))))

(fn GetAttackAnimations
  (params (AnimationSet :type Array%20of%20Anim%20Montage%20Object%20References))
  (bind _output_get (Variables|Animation|SetAttackComboIndex (Math|Integer|%(Integer) (Variables|Animation|GetAttackComboIndex) (Utilities|Array|Length AnimationSet))))
  (Variables|Animation|SetAttackAnimationToPlay (Utilities|Array|Get(acopy) AnimationSet _output_get)))

(fn SetHitAreaLocation)