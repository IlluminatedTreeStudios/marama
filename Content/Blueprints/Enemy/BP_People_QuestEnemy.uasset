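; Child enemy Blueprint for a humanoid quest enemy that fights with a two-step, alternating left and right hand attack combo.
; Construction assigns the attack effect to both hand Niagara glows, which the darkness effect override switches on and off.
; The combo index selects which hand socket the hit area attaches to and which upper-arm socket supplies the end hit location.
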(event EventBeginPlay
  (|CallParentFunction) ; This node is disabled and will not be called.\nDrag off pins to build functionality.
)

(event Collision|EventActorBeginOverlap
  (params (OtherActor :type Actor%20Object%20Reference)))

(event EventTick
  (params (DeltaSeconds :type Float%20%28single-precision%29)))

(fn ConstructionScript
  (|CallParentFunction)
  (Class|NiagaraComponent|SetAsset (Variables|Default|GetNS_LeftHand_Glow) (Variables|Default|GetAttackEffect) true))

(fn AttackToggleDarknessEffect
  (params (On/Off? :type Boolean))
  (bind _ns_lefthand_glow (Variables|Default|GetNS_LeftHand_Glow))
  (if On/Off?
    (Components|Activation|Activate _ns_lefthand_glow false)
    (else
      (Components|Activation|Deactivate _ns_lefthand_glow))))

(fn SetHitAreaLocation
  (if (== (Variables|Default|GetAttackComboIndex) 0) ; 1st Anim
    (Transformation|AttachComponentToComponent (Variables|Default|GetHitArea) (Variables|Character|GetMesh) "LH_S" "KeepRelative" "KeepRelative" "KeepRelative" true)
    (elif (== (Variables|Default|GetAttackComboIndex) 1) ; 2nd Anim
      (Transformation|AttachComponentToComponent (Variables|Default|GetHitArea) (Variables|Character|GetMesh) "RH_S" "KeepRelative" "KeepRelative" "KeepRelative" true))))

(fn GetEndHitLocation
  (Utilities|FlowControl|Sequence
    (:then_0
      (if (== (Variables|Default|GetAttackComboIndex) 0) ; 1st Anim
        (LocalVariables|SetSocket "UpperArm_L")
        (elif (== (Variables|Default|GetAttackComboIndex) 1) ; 2nd Anim
          (LocalVariables|SetSocket "UpperArm_R"))))
    (:then_1
      (return (Transformation|GetSocketLocation (Variables|Character|GetMesh) (LocalVariables|GetSocket))))))