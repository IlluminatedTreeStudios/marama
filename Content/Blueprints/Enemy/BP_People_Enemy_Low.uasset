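; Low-tier human enemy Blueprint, a child that adds a modular head and per-attack hit area placement to its parent enemy class.
; Construction runs the parent script, then applies HeadMesh to the Head skeletal mesh component.
; SetHitAreaLocation replaces the parent logic, attaching HitArea to the left-hand socket for the first combo attack and the right-hand socket for the second.
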(fn ConstructionScript
  (|CallParentFunction)
  (Class|SkinnedMeshComponent|SetSkeletalMesh (Variables|Default|GetHead) (Variables|Mesh|GetHeadMesh) true))

(fn SetHitAreaLocation
  (if (== (Variables|Default|GetAttackComboIndex) 0) ; 1st Anim
    (Transformation|AttachComponentToComponent (Variables|Default|GetHitArea) (Variables|Character|GetMesh) "LH_S" "KeepRelative" "KeepRelative" "KeepRelative" true)
    (elif (== (Variables|Default|GetAttackComboIndex) 1) ; 2nd Anim
      (Transformation|AttachComponentToComponent (Variables|Default|GetHitArea) (Variables|Character|GetMesh) "RH_S" "KeepRelative" "KeepRelative" "KeepRelative" true))))