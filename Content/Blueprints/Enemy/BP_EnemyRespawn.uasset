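; BP_EnemyRespawn is an actor that respawns enemies after a delay, handling several pending respawns at once.
; RespawnEnemy queues an enemy class and time, starting one shared looping half-second timer that counts down every entry.
; Expired entries spawn at random reachable points within the RespawnRadius sphere, receiving this actor as RespawnActor.
; Spawned entries are removed with index adjustment, and the timer clears once the queue is empty.
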(event Custom|RespawnEnemy
  (params (RespawnInfo :type S%20Enemy%20Respawn%20Structure))
  ;[1 1 1] Complex Respawn Function - Handles Multiple Respawns
  (Utilities|Array|Add (Variables|Default|GetRespawnList) RespawnInfo)
  (if (not (Utilities|Time|IsValidTimerHandle (Variables|Default|GetRespawnTimer)))
    (bind _returnvalue (Utilities|Time|SetTimerbyEvent (delegate Custom|RespawnTick) 0.5 true))
    (Variables|Default|SetRespawnTimer _returnvalue)))

(event Custom|RespawnTick
  (bind _indicestospawn (Variables|Default|GetIndicesToSpawn))
  ;[1 1 1] Complex Respawn Function - Handles Multiple Respawns
  (for (_array_element _array_index) (Variables|Default|GetRespawnList)
    (if (> (- (.time _array_element) 0.5) 0.0)
      (Utilities|Array|SetArrayElem (Variables|Default|GetRespawnList) _array_index (Utilities|Struct|MakeS_EnemyRespawn (- (.time _array_element) 0.5) (.enemy _array_element)))
      (else
        (Utilities|Array|Add (Variables|Default|GetIndicesToSpawn) _array_index))))
  (for _array_element_2 (Variables|Default|GetIndicesToSpawn)
    (Game|SpawnActorfromClass (.Enemy (Utilities|Struct|BreakS_EnemyRespawn (Utilities|Array|Get(acopy) (Variables|Default|GetRespawnList) _array_element_2))) (Math|Transform|MakeTransform (.RandomLocation (AI|Navigation|GetRandomReachablePointinRadius (Transformation|GetActorLocation) (Variables|/Script/Engine.SphereComponent|GetSphereRadius (Variables|Default|GetRespawnRadius)) 0 0)) "0, 0, 0" "1,1,1") "AdjustIfPossibleButAlwaysSpawn" 0 self 0)
    (Utilities|Array|RemoveIndex (Variables|Default|GetRespawnList) _array_element_2)
    (for _index (range _array_element_2 (Utilities|Array|LastIndex (Variables|Default|GetIndicesToSpawn)))
      (Utilities|Array|SetArrayElem _indicestospawn _index (- (Utilities|Array|Get(acopy) _indicestospawn _index) 1))))
  (Utilities|Array|Clear (Variables|Default|GetIndicesToSpawn))
  (if (not (> (Utilities|Array|Length (Variables|Default|GetRespawnList)) 0))
    (Utilities|Time|ClearandInvalidateTimerbyHandle (Variables|Default|GetRespawnTimer))))

(event EventBeginPlay)

(event Collision|EventActorBeginOverlap
  (params (OtherActor :type Actor%20Object%20Reference)))

(event EventTick
  (params (DeltaSeconds :type Float%20%28single-precision%29)))

(fn ConstructionScript)